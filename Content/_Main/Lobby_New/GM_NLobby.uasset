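; Lobby game mode that tracks connected players and moves the session to MapVillage on launch via server travel.
; On login it triggers each PC_NLobby's spawn setup; when a player finishes init, it pushes everyone's PlayerInfo to every controller's lobby HUD.
; Helpers rebuild the player and info lists from the GameState PlayerArray on each call.
; The logout handler is empty, so departures do not refresh the HUD.
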(event Custom|LaunchGame
  (Development|ExecuteConsoleCommand "serverTravel MapVillage" 0))

(event Custom|OnPlayerDoneInit
  (params (NewPlayer :type PC%20N%20Lobby%20Object%20Reference))
  (bind _playersinfos (CallFunction|GetAllPlayerInfo))
  (for _array_element (CallFunction|GetAllPlayers)
    (Default|ActLobbyHUD _array_element _playersinfos))
  (Development|PrintString (Utilities|String|ToString(Integer) (Utilities|Array|Length _playersinfos))))

(event EventBeginPlay)

(event EventTick
  (params (DeltaSeconds :type Float%20%28single-precision%29)))

(event EventOnLogout
  (params (ExitingController :type Controller%20Object%20Reference)))

(event EventPostLogin
  (params (NewPlayer :type Player%20Controller%20Object%20Reference))
  (bind _aspc_nlobby (Utilities|Casting|CastToPC_NLobby NewPlayer))
  (Default|OnPlayerSpawn _aspc_nlobby))

(fn ConstructionScript)

(fn GetAllPlayers
  (Utilities|Array|Clear (LocalVariables|GetPlayerListLocal))
  (for _array_element (Variables|/Script/Engine.GameStateBase|GetPlayerArray (Game|GetGameState))
    (bind _aspc_nlobby (Utilities|Casting|CastToPC_NLobby (Game|GetPlayerController _array_element)))
    (Utilities|Array|AddUnique (LocalVariables|GetPlayerListLocal) _aspc_nlobby))
  (return (LocalVariables|GetPlayerListLocal)))

(fn GetAllPlayerInfo
  (Utilities|Array|Clear (LocalVariables|GetPlayerListLocal))
  (for _array_element (CallFunction|GetAllPlayers)
    (Utilities|Array|Add (LocalVariables|GetPlayerListLocal) (Variables|/Game/_Main/Lobby_New/PC_NLobby.PC_NLobby_C|GetPlayerInfo _array_element)))
  (return (LocalVariables|GetPlayerListLocal)))