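; Player controller for the menu that sets up the menu HUD and an options widget.
; BeginPlay calls BeginPlayClient, and the BeginPlay_Client event creates both widgets, adding only the HUD to the viewport.
; The P key toggles the options widget through a FlipFlop, adding it to or removing it from the viewport after validity checks.
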(event Custom|BeginPlay_Client
  ;[1 0.3333 0] Comment
  (bind _returnvalue (UserInterface|CreateWidget "/Game/_Main/Menu/Widgets/HUD_Menu.HUD_Menu_C"))
  (bind _output_get (Variables|Default|SetHUD _returnvalue))
  (UserInterface|Viewport|AddtoViewport _output_get 0)
  (bind _returnvalue_2 (UserInterface|CreateWidget "/Game/_Main/Widget_Options.Widget_Options_C" self))
  (Variables|Default|SetHUD_Menu _returnvalue_2))

(event EventBeginPlay
  (CallFunction|BeginPlayClient))

(event EventTick
  (params (DeltaSeconds :type Float%20%28single-precision%29)))

(event Input|KeyboardEvents|P
  (params (Key :type Key%20Structure))
  (bind _hud_menu (Variables|Default|GetHUD_Menu))
  (bind _hud_menu_2 (Variables|Default|GetHUD_Menu))
  ;[0.7925 0 1] Menu
  (:Pressed
    (Utilities|FlowControl|FlipFlop
      (:A
        (Utilities|IsValid _hud_menu_2
          (:Is%20Valid
            (if (not (UserInterface|Viewport|IsinViewport _hud_menu_2))
              (UserInterface|Viewport|AddtoViewport _hud_menu_2 0)))))
      (:B
        (Utilities|IsValid _hud_menu
          (:Is%20Valid
            (Widget|RemovefromParent _hud_menu)))))))

(event Input|KeyboardEvents|A
  (params (Key :type Key%20Structure)))

(fn ConstructionScript)