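; BP_Field is a box volume actor that registers itself with the heat component of actors inside it.
; On the authority, Box begin overlap adds the field uniquely to the Boxes array of the other actor's BPC_Heat, and end overlap removes it.
; Actors without that component are ignored, and the field applies no effect of its own.
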(event OnComponentBeginOverlap(Box)
  (params (OverlappedComponent :type Primitive%20Component%20Object%20Reference) (OtherActor :type Actor%20Object%20Reference) (OtherComp :type Primitive%20Component%20Object%20Reference) (OtherBodyIndex :type Integer) (bFromSweep :type Boolean) (SweepResult :type Hit%20Result%20Structure%20%28by%20ref%29))
  (bind _returnvalue (Actor|GetComponentbyClass OtherActor "/Game/_Main/Game/Components/BPC_Heat.BPC_Heat_C"))
  (Networking|SwitchHasAuthority
    (:Authority
      (Utilities|IsValid _returnvalue
        (:Is%20Valid
          (Utilities|Array|AddUnique (Variables|/Game/_Main/Game/Components/BPC_Heat.BPC_Heat_C|GetBoxes _returnvalue) self))))))

(event OnComponentEndOverlap(Box)
  (params (OverlappedComponent :type Primitive%20Component%20Object%20Reference) (OtherActor :type Actor%20Object%20Reference) (OtherComp :type Primitive%20Component%20Object%20Reference) (OtherBodyIndex :type Integer))
  (bind _returnvalue (Actor|GetComponentbyClass OtherActor "/Game/_Main/Game/Components/BPC_Heat.BPC_Heat_C"))
  (Networking|SwitchHasAuthority
    (:Authority
      (Utilities|IsValid _returnvalue
        (:Is%20Valid
          (Utilities|Array|RemoveItem (Variables|/Game/_Main/Game/Components/BPC_Heat.BPC_Heat_C|GetBoxes _returnvalue) self))))))

(event EventBeginPlay)

(event Collision|EventActorBeginOverlap
  (params (OtherActor :type Actor%20Object%20Reference)))

(event EventTick
  (params (DeltaSeconds :type Float%20%28single-precision%29)))

(fn ConstructionScript)