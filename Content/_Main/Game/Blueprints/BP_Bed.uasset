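; Possessable bed that lets a player sleep, with look-around controls and Space to wake.
; On interaction the server possesses the bed with the player's controller, and a multicast shows the sleeper's mesh on it.
; A timeline drives a material-parameter "Sleepness" value; its forward finish starts deep sleep, where server ticks shift two player states oppositely.
; Waking reverses the timeline, then returns possession and hides the mesh.
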(event Custom|Wake_Server
  ;[1 0.3647 0] Wake
  (Pawn|Possess (Pawn|GetController) (Variables|Default|GetPCC_PlayerSleeping))
  (Default|WakeServer (Variables|Default|GetPCC_PlayerSleeping))
  (Variables|Default|SetPCC_PlayerSleeping 0)
  (CallFunction|WakeMulticast))

(event Custom|StartSleep
  ;[0.3471 0 1] Try sleeping client only
  (bind (_direction _newtrack_0) (Timeline|GoingDeepSleep Play)
    (:Update
      (Rendering|Material|SetScalarParameterValue "/Game/_Main/Game/MaterialParameterCollections/MPC_Testing.MPC_Testing" "Sleepness" _newtrack_0 :!class /Script/Engine.KismetMaterialLibrary))
    (:Finished
      (switch Utilities|FlowControl|Switch|SwitchonETimelineDirection _direction
        (:Forward
          (CallFunction|SetSleepServer true))
        (:Backward
          (CallFunction|WakeServer))))))

(event Custom|Sleep_Server
  (params (Player :type PCC%20Game%20Object%20Reference))
  ;[0 0.02138 1] Sleep
  (bind _output_get (Variables|Default|SetPCC_PlayerSleeping Player))
  (Pawn|Possess (Pawn|GetController _output_get) self)
  (CallFunction|SleepClient)
  (CallFunction|SleepMulticast (Variables|Default|GetPCC_PlayerSleeping)))

(event Custom|Sleep_Client
  ;[0 0.02138 1] Sleep
  (Pawn|SetControlRotation (Pawn|GetController) (Math|Rotator|MakeRotator 0.0 0.0 1.8e+02)))

(event Custom|Wake_Multicast
  ;[1 0.3647 0] Wake
  (Rendering|SetVisibility (Variables|Default|GetSkeletalMesh) false false))

(event Custom|Sleep_Multicast
  (params (PCC_PlayerSleeping :type PCC%20Game%20Object%20Reference))
  ;[0 0.02138 1] Sleep
  (Utilities|IsValid PCC_PlayerSleeping
    (:Is%20Valid
      (Class|SkinnedMeshComponent|SetSkeletalMesh (Variables|Default|GetSkeletalMesh) (Variables|/Script/Engine.SkinnedMeshComponent|GetSkeletalMesh (Variables|/Script/Engine.Character|GetMesh PCC_PlayerSleeping)) true)
      (Rendering|SetVisibility (Variables|Default|GetSkeletalMesh) true false))
    (:Is%20Not%20Valid
      (Rendering|SetVisibility (Variables|Default|GetSkeletalMesh) false false))))

(event Custom|StartWake
  ;[0.3471 0 1] Try sleeping client only
  (CallFunction|SetSleepServer false)
  (bind (_direction _newtrack_0) (Timeline|GoingDeepSleep Reverse)
    (:Update
      (Rendering|Material|SetScalarParameterValue "/Game/_Main/Game/MaterialParameterCollections/MPC_Testing.MPC_Testing" "Sleepness" _newtrack_0 :!class /Script/Engine.KismetMaterialLibrary))
    (:Finished
      (switch Utilities|FlowControl|Switch|SwitchonETimelineDirection _direction
        (:Forward
          (CallFunction|SetSleepServer true))
        (:Backward
          (CallFunction|WakeServer))))))

(event Custom|SetSleep_Server
  (params (InDeepSleep :type Boolean))
  ;[0 0.001927 0.1927] Deep sleeping
  (Variables|Default|SetInDeepSleep InDeepSleep))

(event Custom|SleepTick_Server
  (bind _pcc_playersleeping (Variables|Default|GetPCC_PlayerSleeping))
  (bind _sleepspeed (Variables|Default|GetSleepSpeed))
  ;[0 0.001927 0.1927] Deep sleeping
  (if (Variables|Default|GetInDeepSleep)
    (Default|AddtoState _pcc_playersleeping "NewEnumerator2" _sleepspeed)
    (Default|AddtoState _pcc_playersleeping "NewEnumerator3" (* _sleepspeed -1.0))))

(event EventBeginPlay)

(event Collision|EventActorBeginOverlap
  (params (OtherActor :type Actor%20Object%20Reference)))

(event EventTick
  (params (DeltaSeconds :type Float%20%28single-precision%29))
  (CallFunction|SleepTickServer))

(event EventOnMainInteraction
  (params (Player :type PCC%20Game%20Object%20Reference))
  ;[1 0.006586 0] Actions
  (Utilities|IsValid (Variables|Default|GetPCC_PlayerSleeping)
    (:Is%20Not%20Valid
      (CallFunction|SleepServer Player)
      (Default|SleepServer Player)
      (CallFunction|StartSleep))))

(event Input|AxisEvents|InputAxisLookUp
  (params (AxisValue :type Float%20%28single-precision%29))
  ;[0.162 0 1] Controles
  (Pawn|Input|AddControllerPitchInput AxisValue))

(event Input|AxisEvents|InputAxisLookRight
  (params (AxisValue :type Float%20%28single-precision%29))
  ;[0.162 0 1] Controles
  (Pawn|Input|AddControllerYawInput AxisValue))

(event Input|KeyboardEvents|SpaceBar
  (params (Key :type Key%20Structure))
  ;[1 0.006586 0] Actions
  (:Pressed
    (CallFunction|StartWake)))

(fn ConstructionScript)