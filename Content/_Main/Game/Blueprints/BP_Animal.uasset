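; BP_Animal is a huntable AI animal that wanders, flees, and drops ham pickups when killed.
; On authority, it picks an interest point at BeginPlay, then roams reachable points around it with random pauses.
; PawnSensing redirects it on seeing a player or hearing noise, using the reversed direction as a world-space position, not offset from the animal.
; Any damage reduces Health; at zero it spawns BP_Eatable_Jambon items and destroys itself.
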(event OnSeePawn(PawnSensing)
  (params (Pawn :type Pawn%20Object%20Reference))
  (bind _aspcc_game (Utilities|Casting|CastToPCC_Game Pawn))
  (CallFunction|Moveto (.RandomLocation (AI|Navigation|GetRandomReachablePointinRadius (* (Math|Vector|Normalize (- (Transformation|GetActorLocation _aspcc_game) (Transformation|GetActorLocation))) -5e+03) 1e+03 0 0))))

(event OnHearNoise(PawnSensing)
  (params (Instigator :type Pawn%20Object%20Reference) (Location :type Vector%20%28by%20ref%29 :default "0, 0, 0") (Volume :type Float%20%28single-precision%29))
  (Development|PrintString "I HEARD !!!")
  (CallFunction|Moveto (.RandomLocation (AI|Navigation|GetRandomReachablePointinRadius (* (Math|Vector|Normalize (- Location (Transformation|GetActorLocation))) -5e+03) 1e+03 0 0))))

(event Custom|Die
  (for _index (range 0 3)
    (Game|SpawnActorfromClass "/Game/_Main/Game/GrabableObjects/Aliments/BP_Eatable_Jambon.BP_Eatable_Jambon_C" (Transformation|GetWorldTransform (Variables|Default|GetScene)) "AdjustIfPossibleButAlwaysSpawn" 0 "/Game/Fantastic_Village_Pack/meshes/props/food/SM_PROP_food_meat_05.SM_PROP_food_meat_05" 1e+01 5e+01 "NewEnumerator1" false true 0))
  (Actor|DestroyActor))

(event Custom|OnTakeAnyDamage_Event_0
  (params (DamagedActor :type Actor%20Object%20Reference) (Damage :type Float%20%28single-precision%29) (DamageType :type Damage%20Type%20Object%20Reference) (InstigatedBy :type Controller%20Object%20Reference) (DamageCauser :type Actor%20Object%20Reference))
  (CallFunction|TakeDamages Damage))

(event Custom|TakeDamages
  (params (B :type Float%20%28double-precision%29))
  (bind _output_get (Variables|Default|SetHealth (- (Variables|Default|GetHealth) B)))
  (if (<= _output_get 0.0)
    (CallFunction|Die)))

(event Custom|MoveTo
  (params (Destination :type Vector))
  (AI|AIMoveTo self Destination 0 5.0 false
    (:OnSuccess
      (Utilities|FlowControl|Delay (* (Math|Random|RandomFloat) 5.0))
      (CallFunction|Moveto (.RandomLocation (AI|Navigation|GetRandomReachablePointinRadius (Variables|Default|GetIntrerestPoint) 1e+03 0 0))))))

(event Custom|SetNewIntrestPoint
  (Variables|Default|SetIntrerestPoint (.RandomLocation (AI|Navigation|GetRandomReachablePointinRadius (Transformation|GetActorLocation) 1e+05 0 0))))

(event EventBeginPlay
  (EventDispatchers|AssignOnTakeAnyDamage (delegate Custom|OnTakeAnyDamage_Event_0))
  (Networking|SwitchHasAuthority
    (:Authority
      (CallFunction|SetNewIntrestPoint)
      (CallFunction|Moveto (.RandomLocation (AI|Navigation|GetRandomReachablePointinRadius (Variables|Default|GetIntrerestPoint) 1e+04 0 0))))))

(event Collision|EventActorBeginOverlap
  (params (OtherActor :type Actor%20Object%20Reference)))

(event EventTick
  (params (DeltaSeconds :type Float%20%28single-precision%29)))

(fn ConstructionScript)