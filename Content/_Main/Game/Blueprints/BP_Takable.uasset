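; BP_Takable is a networked physics item that characters can grab, drop, throw and use with a cooldown.
; Multicast events toggle physics and collision profiles, attaching the mesh to the character's left or two-hand component with an offset derived from GrabPoint.
; One-handed grabs can hide the mesh in third person in favor of an in-hand model.
; BPCHeat temperature changes drive a dynamic material's Heat parameter.
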(event Custom|Used_Server
  (params (By :type PCC%20Game%20Object%20Reference))
  (Development|PrintString "Object used"))

(event Custom|Grabed_Multicast
  (params (Character :type PCC%20Game%20Object%20Reference))
  ;[1 0 0.5903 0.2] Take
  (Variables|Default|SetGraber Character)
  (if (Utilities|Enum|Equal(Enum) (Variables|Default|GetHand) "NewEnumerator2")
    (CallFunction|SetMode false)
    (Transformation|AttachComponentToComponent (Variables|Default|GetStaticMesh) (Variables|/Game/_Main/Game/Characters/PCC_Game.PCC_Game_C|GetTwoHands (Variables|Default|GetGraber)) "" "SnapToTarget" "SnapToTarget" "SnapToTarget" true)
    (Transformation|SetRelativeTransform (Variables|Default|GetStaticMesh) (Variables|Default|GetHandOffset) false false)
    (Default|SetHandContent (Variables|Default|GetGraber))
    (else
      ;;[1 0.1989 0] All
      (CallFunction|SetMode false)
      (Transformation|AttachComponentToComponent (Variables|Default|GetStaticMesh) (Variables|/Game/_Main/Game/Characters/PCC_Game.PCC_Game_C|GetLeftHand (Variables|Default|GetGraber)) "" "SnapToTarget" "SnapToTarget" "SnapToTarget" true)
      (Transformation|SetRelativeTransform (Variables|Default|GetStaticMesh) (Variables|Default|GetHandOffset) false false)
      (if (not (Default|IsOwnered (Variables|Default|GetGraber)))
        ;;[0.02341 0 1] Third person
        (if (Variables|Default|GetInHandModel?)
          (Rendering|SetVisibility (Variables|Default|GetStaticMesh) false false)
          (Default|SetHandContent (Variables|Default|GetGraber) self))
        (else
          ;;[1 0.3333 0] First person
          (Default|SetHandContent (Variables|Default|GetGraber)))))))

(event Custom|TryUse
  (params (By :type PCC%20Game%20Object%20Reference))
  (Utilities|FlowControl|DoOnce false :!label _label
    (:Completed
      (Utilities|FlowControl|Sequence
        (:then_0
          (CallFunction|UsedServer By))
        (:then_1
          (Utilities|FlowControl|Delay (Variables|Default|GetCooldown))
          (goto _label Reset))))))

(event Custom|Destroy_Server
  (Actor|DestroyActor))

(event Custom|OnTemperatureChanged
  (params (NewTemperature :type Float%20%28double-precision%29))
  (CallFunction|ChangeTexture NewTemperature))

(event Custom|Throwed_Multicast
  (params (Impulse :type Vector))
  (bind _graber (Variables|Default|GetGraber))
  ;[1 0 0.8734] On drop multicast
  (CallFunction|SetMode true)
  (Default|SetHandContent _graber)
  (Variables|/Game/_Main/Game/Characters/PCC_Game.PCC_Game_C|SetInHand _graber 0)
  (Physics|AddImpulse (Variables|Default|GetStaticMesh) Impulse "None" false))

(event Custom|Throwed_Server
  (params (Impulse :type Vector) (Launcher :type PCC%20Game%20Object%20Reference))
  ;[0.09621 0 1] Throwed server
  (CallFunction|ThrowedMulticast Impulse))

(event Custom|SetGravity_Server
  (params (HasGravity :type Boolean))
  ;[1 0 0] Set Gravity
  (CallFunction|SetGravityMulticast HasGravity))

(event Custom|ChangeTexture
  (params (Value :type Float%20%28single-precision%29))
  (bind _material (Variables|Default|GetMaterial))
  (Utilities|IsValid _material
    (:Is%20Valid
      (Rendering|Material|SetScalarParameterValue _material "Heat" Value :!class /Script/Engine.MaterialInstanceDynamic))
    (:Is%20Not%20Valid
      (Development|PrintString (Utilities|GetObjectName self) true true "(R=1.000000,G=0.000000,B=0.000000,A=1.000000)"))))

(event Custom|SetGravity_Multicast
  (params (HasGravity :type Boolean))
  ;[1 0 0] Set Gravity
  (Physics|SetEnableGravity (Variables|Default|GetStaticMesh) HasGravity))

(event Custom|Droped_Multicast
  (bind _graber (Variables|Default|GetGraber))
  ;[1 0 0.8734] On drop multicast
  (CallFunction|SetMode true)
  (Default|SetHandContent _graber)
  (Variables|/Game/_Main/Game/Characters/PCC_Game.PCC_Game_C|SetInHand _graber 0))

(event Custom|BeginPlayServer
  ;[1 0 0] BeginPlay server
  (Variables|Default|SetHandOffset (Math|Transform|InvertTransform (Transformation|GetRelativeTransform (Variables|Default|GetGrabPoint)))))

(event Custom|OnTakeAnyDamage_Event_0
  (params (DamagedActor :type Actor%20Object%20Reference) (Damage :type Float%20%28single-precision%29) (DamageType :type Damage%20Type%20Object%20Reference) (InstigatedBy :type Controller%20Object%20Reference) (DamageCauser :type Actor%20Object%20Reference)))

(event Custom|ChangeState
  (params (NewState :type Integer))
  (Variables|Default|SetState NewState))

(event Custom|ChangeMesh
  (params (NewMesh :type Static%20Mesh%20Object%20Reference))
  ;[0 0.04601 1] Change the mesh
  (Variables|Default|SetMesh NewMesh)
  (CallFunction|ChangeMeshMulticast NewMesh))

(event Custom|DestroySelf
  (bind _graber (Variables|Default|GetGraber))
  ;[0.3152 0 1] Destroy self
  (Variables|/Game/_Main/Game/Characters/PCC_Game.PCC_Game_C|SetInHand _graber 0)
  (CallFunction|DestroySelfMulticast _graber))

(event Custom|ChangeMesh_Multicast
  (params (UpdatedMesh :type Static%20Mesh%20Object%20Reference))
  ;[0 0.04601 1] Change the mesh
  (Default|UpdateHandMesh (Variables|Default|GetGraber) UpdatedMesh))

(event Custom|DestroySelf_Multicast
  (params (Target :type PCC%20Game%20Object%20Reference))
  ;[0.3152 0 1] Destroy self
  (Default|SetHandContent Target)
  (Actor|DestroyActor))

(event EventBeginPlay
  (bind _staticmesh (Variables|Default|GetStaticMesh))
  ;[1 0 0] BeginPlay
  (Utilities|FlowControl|Sequence
    (:then_0
      (Networking|SwitchHasAuthority
        (:Authority
          (CallFunction|BeginPlayServer))
        (:Remote
          _))
      (Transformation|SetRelativeTransform (Variables|Default|GetGrabPoint) (Math|Transform|InvertTransform (Variables|Default|GetHandOffset)) false false))
    (:then_1
      (CallFunction|SetMode true))
    (:then_2
      (EventDispatchers|AssignOnTakeAnyDamage (delegate Custom|OnTakeAnyDamage_Event_0)))
    (:then_3
      ;[0 0.5 0] Set dynamic material
      (bind _returnvalue (Rendering|Material|CreateDynamicMaterialInstance (Rendering|Material|GetMaterial _staticmesh 0) "None" "None" :!class /Script/Engine.KismetMaterialLibrary))
      (bind _output_get (Variables|Default|SetMaterial _returnvalue))
      (Rendering|Material|SetMaterial _staticmesh 0 _output_get)
      (EventDispatchers|BindEventtoOnTemperatureChanged (Variables|Default|GetBPC_Heat) (delegate Custom|OnTemperatureChanged)))))

(event EventOnMainInteraction
  (params (Player :type PCC%20Game%20Object%20Reference))
  (CallFunction|GrabedMulticast Player))

(event EventTick
  (params (DeltaSeconds :type Float%20%28single-precision%29)))

(fn ConstructionScript
  (Components|StaticMesh|SetStaticMesh (Variables|Default|GetStaticMesh) (Variables|Default|GetMesh))
  (Variables|/Script/Engine.ArrowComponent|SetArrowLength (Variables|Default|GetArrow3) (Variables|Default|GetHandLength))
  (Components|Sphere|SetSphereRadius (Variables|Default|GetSphere) (Variables|Default|GetObjectRadius) true))

(fn SetMode
  (params (Sim :type Boolean))
  (bind _staticmesh (Variables|Default|GetStaticMesh))
  (bind _staticmesh_2 (Variables|Default|GetStaticMesh))
  (if Sim
    (Physics|SetSimulatePhysics _staticmesh true)
    (Collision|SetCollisionProfileName _staticmesh (select (Variables|Default|GetHardPlayerCollision) "HardObject" "SoftObject") true :!class /Script/Engine.PrimitiveComponent)
    (Transformation|DetachFromComponent (Variables|Default|GetStaticMesh) "KeepWorld" "KeepWorld" "KeepWorld" true)
    (Rendering|SetVisibility (Variables|Default|GetStaticMesh) true false)
    (else
      (Physics|SetSimulatePhysics _staticmesh_2 false)
      (Collision|SetCollisionProfileName _staticmesh_2 (select (Variables|Default|GetHardPlayerCollision) "GrabedHardObject" "GrabedSoftObject") true :!class /Script/Engine.PrimitiveComponent))))

(fn OnRepMesh
  (Components|StaticMesh|SetStaticMesh (Variables|Default|GetStaticMesh) (Variables|Default|GetMesh)))