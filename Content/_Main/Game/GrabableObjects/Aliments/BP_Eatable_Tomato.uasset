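; Throwable tomato, an eatable grabable object that splashes and is destroyed when it hits something after being thrown.
; The server-side throw event sets a Launched flag before calling the parent throw logic.
; On a component hit, the authority clears the flag, multicasts the splash and destroys the tomato.
; The multicast spawns a potion blub particle effect at the hit location, tinted red.
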(event OnComponentHit(StaticMesh)
  (params (HitComponent :type Primitive%20Component%20Object%20Reference) (OtherActor :type Actor%20Object%20Reference) (OtherComp :type Primitive%20Component%20Object%20Reference) (NormalImpulse :type Vector :default "0, 0, 0") (Hit :type Hit%20Result%20Structure%20%28by%20ref%29))
  (bind (_bblockinghit _binitialoverlap _time _distance _location _impactpoint _normal) (Collision|BreakHitResult Hit))
  (Networking|SwitchHasAuthority
    (:Authority
      (if (Variables|Default|GetLaunched)
        (Variables|Default|SetLaunched false)
        (CallFunction|SplashMulticast _location _normal)
        (CallFunction|DestroyServer)))))

(event Custom|Splash_Multicast
  (params (Hit%20Location :type Vector) (Hit%20Normal :type Vector))
  (bind _returnvalue (Niagara|SpawnSystematLocation "/Game/_Main/Game/Particles/P_PotionBlub.P_PotionBlub" Hit%20Location))
  (Effects|Components|ParticleSystem|SetColorParameter _returnvalue "Color" "(R=1.000000,G=0.000000,B=0.000000,A=1.000000)"))

(event EventBeginPlay
  (|CallParentFunction) ; This node is disabled and will not be called.\nDrag off pins to build functionality.
)

(event Collision|EventActorBeginOverlap
  (params (OtherActor :type Actor%20Object%20Reference))
  (|CallParentFunction OtherActor) ; This node is disabled and will not be called.\nDrag off pins to build functionality.
)

(event EventTick
  (params (DeltaSeconds :type Float%20%28single-precision%29))
  (|CallParentFunction DeltaSeconds) ; This node is disabled and will not be called.\nDrag off pins to build functionality.
)

(event EventThrowedServer
  (params (Impulse :type Vector :default "0, 0, 0") (Launcher :type PCC%20Game%20Object%20Reference))
  (Variables|Default|SetLaunched true)
  (|CallParentFunction Impulse 0))

(fn ConstructionScript
  (|CallParentFunction))