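; BP_Eatable is a grabbable food item that is eaten in stages, restoring hunger to whoever uses it.
; Each server-side use adds Restoration to the user's Hunger and, if they have a heat component, sets its temperature halfway between their target temperature and the food's.
; It then advances State, swapping to the next entry in Meshes and destroying itself once the list runs out.
; The PotionEffect override switches on potion type without any visible effects.
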(event EventBeginPlay
  (|CallParentFunction) ; This node is disabled and will not be called.\nDrag off pins to build functionality.
)

(event Collision|EventActorBeginOverlap
  (params (OtherActor :type Actor%20Object%20Reference)))

(event EventTick
  (params (DeltaSeconds :type Float%20%28single-precision%29))
  (|CallParentFunction DeltaSeconds) ; This node is disabled and will not be called.\nDrag off pins to build functionality.
)

(event EventUsedServer
  (params (By :type PCC%20Game%20Object%20Reference))
  (bind _states (Variables|/Game/_Main/Game/Characters/PCC_Game.PCC_Game_C|GetStates By))
  (|CallParentFunction By)
  (Utilities|Struct|SetmembersinS_PlayerStates _states (+ (.Hunger (Utilities|Struct|BreakS_PlayerStates _states)) (Variables|Default|GetRestoration)))
  (bind _bpc_heat (Variables|/Game/_Main/Game/Characters/PCC_Game.PCC_Game_C|GetBPC_Heat By)
    (:then
      (Variables|/Game/_Main/Game/Components/BPC_Heat.BPC_Heat_C|SetTemperature _bpc_heat (Math|Float|Lerp (Variables|/Game/_Main/Game/Components/BPC_Heat.BPC_Heat_C|GetTargetTemperature _bpc_heat) (Variables|/Game/_Main/Game/Components/BPC_Heat.BPC_Heat_C|GetTemperature (Variables|Default|GetBPC_Heat)) 0.5)))
    (:else
      _))
  (CallFunction|ChangeState (+ (Variables|Default|GetState) 1)))

(event EventChangeState
  (params (NewState :type Integer))
  (bind _meshes (Variables|Default|GetMeshes))
  (|CallParentFunction NewState)
  (if (== (Utilities|Array|Length _meshes) NewState)
    (CallFunction|DestroySelf)
    (else
      (CallFunction|ChangeMesh (Utilities|Array|Get(acopy) _meshes NewState)))))

(event EventPotionEffect
  (params (Potion :type EPotionEffects%20Enum :default "NewEnumerator0") (Percent :type Float%20%28double-precision%29) (Position :type Vector :default "0, 0, 0") (Causer :type PCC%20Game%20Object%20Reference))
  (switch Utilities|FlowControl|Switch|SwitchonEPotionEffects Potion))

(fn ConstructionScript
  (|CallParentFunction))