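; BP_Potion is a grabbable potion bottle that starts empty and can be filled with a potion class, then splashed.
; Server fill and empty events set the class and multicast material updates for fill state and color.
; A server splash sphere-traces at the hit, applies the potion object once per blocking-hit actor, then destroys the bottle.
; The splash multicast spawns Niagara effects and sound from the potion's class defaults.
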(event Custom|FillPotion_Server
  (params (Potion :type Potion%20Class%20Reference))
  ;[0.03505 1 0] Fill
  (bind _output_get (Variables|Default|SetPotion Potion))
  (CallFunction|FillPotionMulticast _output_get))

(event Custom|FillPotion_Multicast
  (params (Potion :type Potion%20Class%20Reference))
  (bind _material (Variables|Default|GetMaterial))
  ;[0.03505 1 0] Fill
  (Rendering|Material|SetScalarParameterValue _material "Filled" 1.0 :!class /Script/Engine.MaterialInstanceDynamic)
  (Rendering|Material|SetVectorParameterValue _material "PotionColor" (.Color (Utilities|GetClassDefaults Potion)) :!class /Script/Engine.MaterialInstanceDynamic))

(event Custom|Empty_Server
  ;[1 0.3118 0] Empty
  (Variables|Default|SetPotion 0)
  (CallFunction|EmptyMulticast))

(event Custom|Empty_Multicast
  ;[1 0.3118 0] Empty
  (Rendering|Material|SetScalarParameterValue (Variables|Default|GetMaterial) "Filled" 0.0 :!class /Script/Engine.MaterialInstanceDynamic))

(event EventBeginPlay
  (|CallParentFunction)
  (CallFunction|EmptyServer))

(event Collision|EventActorBeginOverlap
  (params (OtherActor :type Actor%20Object%20Reference))
  (|CallParentFunction OtherActor) ; This node is disabled and will not be called.\nDrag off pins to build functionality.
)

(event EventTick
  (params (DeltaSeconds :type Float%20%28single-precision%29))
  (|CallParentFunction DeltaSeconds) ; This node is disabled and will not be called.\nDrag off pins to build functionality.
)

(event EventSplashMulticast
  (params (SplashLocation :type Vector :default "0, 0, 0") (SplashNormal :type Vector :default "0, 0, 0"))
  (bind _potion (Variables|Default|GetPotion))
  (bind (_splasheffect _color _coockedeffect _sound) (Utilities|GetClassDefaults _potion))
  ;[1 1 0] Splash multicast
  (if (Utilities|IsValidClass _potion)
    (bind _returnvalue (Niagara|SpawnSystematLocation _splasheffect SplashLocation (Math|Rotator|MakeRotfromZ SplashNormal)))
    (Effects|Components|ParticleSystem|SetColorParameter _returnvalue "Color" _color)
    (Audio|PlaySoundatLocation _sound SplashLocation "0, 0, 0" 1.0 1.0 0.0 "/Game/_Main/Game/Audios/SA_Basic.SA_Basic" 0 0 0)))

(event EventSplashServer
  (params (HitLocation :type Vector :default "0, 0, 0") (HitNormal :type Vector :default "0, 0, 0"))
  (bind _allreadyaffectedactors (Variables|Default|GetAllreadyAffectedActors))
  (bind _potion (Variables|Default|GetPotion))
  ;[0.08872 0 1] Splash on server
  (|CallParentFunction HitLocation HitNormal)
  (if (Utilities|IsValidClass _potion)
    (bind _outhits (Collision|MultiSphereTraceByChannel HitLocation HitLocation (Variables|Default|GetRadius) "TraceTypeQuery1" false 0 "None"))
    (bind _returnvalue (Game|ConstructObjectfromClass _potion))
    (Utilities|Set|Clear (Variables|Default|GetAllreadyAffectedActors))
    (for _array_element _outhits
      (if (.bBlockingHit (Collision|BreakHitResult _array_element))
        (if (not (Utilities|Set|Contains _allreadyaffectedactors (.HitActor (Collision|BreakHitResult _array_element))))
          (Utilities|Set|Add _allreadyaffectedactors (.HitActor (Collision|BreakHitResult _array_element)))
          (Default|ObjectSplashed _returnvalue (.HitActor (Collision|BreakHitResult _array_element)) 1.0 (.ImpactPoint (Collision|BreakHitResult _array_element)) (Variables|Default|GetLauncher)))))
    (Actor|DestroyActor)))

(fn ConstructionScript
  (|CallParentFunction))

(fn ForEachOnce)