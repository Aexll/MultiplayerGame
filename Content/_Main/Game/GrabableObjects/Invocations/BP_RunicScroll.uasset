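; BP_RunicScroll is a runic scroll Blueprint that displays a stone index through its material and can invoke an incantation.
; BeginPlay applies StoneIndex to the material's Index scalar parameter.
; The Force parameter is set directly or animated by the Exited timeline, which plays forward on StartExited and reverses on StopExited.
; Invoke constructs an object from the Incantation class and calls its Invoke.
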(event Custom|SetStoneIndex
  (params (Index :type Integer))
  (bind _material (Variables|Default|GetMaterial))
  (Utilities|IsValid _material
    (:Is%20Valid
      (Rendering|Material|SetScalarParameterValue _material "Index" (Math|Conversions|ToFloat(Integer) Index) :!class /Script/Engine.MaterialInstanceDynamic))))

(event Custom|SetForce
  (params (Force :type Float%20%28double-precision%29))
  (Rendering|Material|SetScalarParameterValue (Variables|Default|GetMaterial) "Force" Force :!class /Script/Engine.MaterialInstanceDynamic))

(event Custom|StartExited
  (bind _newtrack_0 (Timeline|Exited Play)
    (:Update
      (CallFunction|SetExited _newtrack_0))))

(event Custom|StopExited
  (bind _newtrack_0 (Timeline|Exited Reverse)
    (:Update
      (CallFunction|SetExited _newtrack_0))))

(event Custom|SetExited
  (params (Exitement :type Float%20%28double-precision%29))
  (Rendering|Material|SetScalarParameterValue (Variables|Default|GetMaterial) "Force" Exitement :!class /Script/Engine.MaterialInstanceDynamic))

(event Custom|Invoke
  (bind _returnvalue (Game|ConstructObjectfromClass (Variables|Default|GetIncantation)))
  (Default|Invoke _returnvalue))

(event EventBeginPlay
  (|CallParentFunction)
  (CallFunction|SetStoneIndex (Variables|ServerOnly|GetStoneIndex)))

(event Collision|EventActorBeginOverlap
  (params (OtherActor :type Actor%20Object%20Reference)))

(event EventTick
  (params (DeltaSeconds :type Float%20%28single-precision%29))
  (|CallParentFunction DeltaSeconds) ; This node is disabled and will not be called.\nDrag off pins to build functionality.
)

(fn ConstructionScript
  (|CallParentFunction))