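; Heat component that simulates its owner's temperature, applying cold or fire damage at extremes.
; On authority, Tick lerps temperature toward the last heat box in its list, or the GameState's ambient values when there is none, then pushes changes through events.
; For BP_Takable owners, it attaches a fire effect scaled to object radius, toggled by multicast according to a burning threshold.
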(event Custom|Client
  (params (InDouble :type Float%20%28double-precision%29))
  (bind _output_get (Variables|Default|SetTemperature InDouble)))

(event Custom|Multicast
  (params (Burning? :type Boolean))
  (bind _fireeffect (Variables|Default|GetFireEffect)
    (:then
      (if Burning?
        (Components|Activation|Activate _fireeffect false)
        (else
          (Components|Activation|Deactivate _fireeffect))))
    (:else)))

(event Custom|BeginPlayClient
  (params (Target :type BP%20Takable%20Object%20Reference))
  (bind _returnvalue (Niagara|SpawnSystemAttached "/Game/_Main/Game/Particles/P_FireTest.P_FireTest" (Variables|/Game/_Main/Game/Blueprints/BP_Takable.BP_Takable_C|GetStaticMesh Target) "None" "0, 0, 0" "0, 0, 0" "KeepRelativeOffset" false false))
  (bind _output_get (Variables|Default|SetFireEffect _returnvalue))
  (Effects|Components|ParticleSystem|SetFloatParameter _output_get "FireSize" (/ (Variables|/Game/_Main/Game/Blueprints/BP_Takable.BP_Takable_C|GetObjectRadius Target) 14.0)))

(event EventBeginPlay
  (Components|Tick|SetComponentTickEnabled (Ability|HasAuthority (Components|GetOwner)))
  (bind _output_get (Variables|Default|SetTemperature (.AmbianteTemperature (CallFunction|GetAmbianteTemperature))))
  (CallFunction|Client _output_get)
  (bind _asbp_takable (Utilities|Casting|CastToBP_Takable (Components|GetOwner)))
  (CallFunction|BeginPlayClient _asbp_takable))

(event EventTick
  (params (DeltaSeconds :type Float%20%28single-precision%29))
  (bind _returnvalue (Components|GetOwner))
  (bind (_ambiantetemperature _ambiantdiffusion) (CallFunction|GetAmbianteTemperature))
  (bind _boxes (Variables|Default|GetBoxes))
  (bind _returnvalue_2 (Utilities|Array|LastIndex _boxes))
  (bind _output (Utilities|Array|Get(acopy) _boxes _returnvalue_2))
  (Utilities|IsValid _output
    (:Is%20Valid
      (Variables|Default|SetTargetTemperature (Variables|/Game/_Main/Game/Blueprints/BP_Field.BP_Field_C|GetTemperature _output))
      (Variables|Default|SetTargetDiffusion (Variables|/Game/_Main/Game/Blueprints/BP_Field.BP_Field_C|GetDiffusion _output)))
    (:Is%20Not%20Valid
      (Variables|Default|SetTargetTemperature _ambiantetemperature)
      (Variables|Default|SetTargetDiffusion _ambiantdiffusion)))
  (if (!= (Variables|Default|GetTemperature) (Variables|Default|GetTargetTemperature))
    (bind _output_get (Variables|Default|SetTemperature (CallFunction|LerpTillTresshold (Variables|Default|GetTemperature) (Variables|Default|GetTargetTemperature) (/ (Variables|Default|GetTargetDiffusion) 1e+02) 0.1)))
    (CallFunction|Client _output_get)
    (Default|CallOnTemperatureChanged _output_get)
    (if (< (Variables|Default|GetTemperature) 0.0)
      (Game|Damage|ApplyDamage _returnvalue (/ (Variables|Default|GetTemperature) -1e+03) 0 0 "/Game/_Main/Game/DamageTypes/DMG_Cold.DMG_Cold_C")
      (elif (> (Variables|Default|GetTemperature) 1e+02)
        (Game|Damage|ApplyDamage _returnvalue (/ (- (Variables|Default|GetTemperature) 5e+01) 1e+03) 0 0 "/Game/_Main/Game/DamageTypes/DMG_Fire.DMG_Fire_C")
        (CallFunction|Multicast (> (Variables|Default|GetTemperature) 1.5e+02))))))

(fn GetAmbianteTemperature
  (Utilities|IsValid (Variables|World|GetGS)
    (:Is%20Valid
      _)
    (:Is%20Not%20Valid
      (bind _asgs (Utilities|Casting|CastToGS_Game (Game|GetGameState))
        (:then
          (Variables|World|SetGS _asgs))
        (:CastFailed
          (return 19.0 0.5)))))
  (return (Variables|/Game/_Main/Game/GS_Game.GS_Game_C|GetAmbianteTemperature (Variables|World|GetGS)) (Variables|/Game/_Main/Game/GS_Game.GS_Game_C|GetAmbiantDiffusion (Variables|World|GetGS))))