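; Player controller for a role-based game with days and a village win/lose outcome, owning the player's HUD widgets.
; BeginPlay creates the main HUD and a menu, which M toggles along with cursor and input mode.
; Events drive the loading screen, then pass role reveal, new day (via NewDayClient) and game end to the main HUD.
; R has GM_Game reassign roles and reset players.
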(event Custom|ShowLoadingScreen
  ;[0 0.3177 0.04996] Loading Screen
  (bind _hud_loading (Variables|Default|GetHUD_Loading)
    (:then
      (if (UserInterface|Viewport|IsinViewport _hud_loading)
        (UserInterface|Viewport|AddtoViewport _hud_loading 1 :!label _label)
        (Default|StartLoading _hud_loading)))
    (:else
      (bind _returnvalue (UserInterface|CreateWidget "/Game/_Main/Game/Widgets/HUD_Loading.HUD_Loading_C" self))
      (Variables|Default|SetHUD_Loading _returnvalue)
      (goto _label))))

(event Custom|GenerateHUD
  ;[0.0771 0 1] HUDs init
  (bind _returnvalue (UserInterface|CreateWidget "/Game/_Main/Game/Widgets/HUD_MainGame.HUD_MainGame_C" self))
  (bind _output_get (Variables|Default|SetHUD_Game _returnvalue))
  (UserInterface|Viewport|AddtoViewport _output_get 0)
  (bind _returnvalue_2 (UserInterface|CreateWidget "/Game/_Main/HUD_Menu.HUD_Menu_C" self))
  (Variables|Default|SetHUD_Menu _returnvalue_2))

(event Custom|RemoveLoadingScreenAfter
  (params (Time :type Float%20%28double-precision%29))
  ;[0 0.3177 0.04996] Loading Screen
  (bind _hud_loading (Variables|Default|GetHUD_Loading)
    (:then
      (if (UserInterface|Viewport|IsinViewport _hud_loading)
        (Default|DoneLoading _hud_loading Time)
        (Utilities|FlowControl|Delay Time)
        (CallFunction|ShowRoleHUD)))
    (:else)))

(event Custom|ShowRoleHUD
  ;[0 1 0.1234] Role HUD
  (bind _hud_game (Variables|Default|GetHUD_Game)
    (:then
      (Default|ShowRole _hud_game (Variables|Default|GetPlayerRole)))
    (:else)))

(event Custom|NewDayClient
  (params (DoomdayIn :type Integer))
  (Default|NewDayStart (Variables|Default|GetHUD_Game) DoomdayIn))

(event Custom|PlayerEndGame
  (params (VillageWin :type Boolean))
  (Variables|Default|SetbShowMouseCursor true)
  (Default|GameEnd (Variables|Default|GetHUD_Game) VillageWin))

(event Custom|RestartAllPlayers
  ;[1 0 0.366] Possess
  (bind _asgm (Utilities|Casting|CastToGM_Game (Game|GetGameMode)))
  (Default|SetPlayersRoles _asgm)
  (Default|ResetPlayers _asgm))

(event EventBeginPlay
  (CallFunction|GenerateHUD))

(event EventTick
  (params (DeltaSeconds :type Float%20%28single-precision%29)))

(event EventPossess
  (params (PossessedPawn :type Pawn%20Object%20Reference))
  ;[1 0 0.366] Possess
)

(event EventUnPossess
  (params (UnpossessedPawn :type Pawn%20Object%20Reference))
  ;[1 0 0.366] Possess
)

(event EventNewDayStart
  (params (DoomdayIn :type Integer))
  (CallFunction|NewDayClient DoomdayIn))

(event Input|KeyboardEvents|R
  (params (Key :type Key%20Structure))
  ;[1 0 0.366] Possess
  (:Pressed
    (CallFunction|RestartAllPlayers)))

(event Input|KeyboardEvents|M
  (params (Key :type Key%20Structure))
  ;[1 0.526 0.1335] Open Menu
  (:Pressed
    (bind _hud_menu (Variables|Default|GetHUD_Menu)
      (:then
        (if (UserInterface|Viewport|IsinViewport _hud_menu)
          (Widget|RemovefromParent _hud_menu)
          (Variables|Default|SetbShowMouseCursor false)
          (Input|SetInputModeGameOnly self)
          (else
            (UserInterface|Viewport|AddtoViewport _hud_menu 0)
            (Variables|Default|SetbShowMouseCursor true)
            (UserInterface|Animation|PlayAnimation _hud_menu (Variables|/Game/_Main/HUD_Menu.HUD_Menu_C|GetOpenMenu _hud_menu) 0.0 1 "Forward" 1.0 true)
            (Input|SetInputModeGameandUI self (Variables|Default|GetHUD_Menu) "DoNotLock" false))))
      (:else
        (Development|PrintString "Unvalid HUD menu" true true "(R=1.000000,G=0.000000,B=0.000000,A=1.000000)" 1e+02)))))

(fn ConstructionScript)