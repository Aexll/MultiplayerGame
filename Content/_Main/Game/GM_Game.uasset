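; Game mode for a village hidden-killer game: sets up roles, houses and player pawns, and relays the win result to controllers.
; Outside debug, a delayed BeginPlay draws roles from a pool without repeats, picks one random killer, then resets players and sets morning time.
; Reset spawns role-specific houses for shuffled players at indexed spawnpoints, mapped by controller.
; Each player then respawns at their house, falling back to role-tagged or default PlayerStarts.
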(event Custom|SetPlayersRoles
  ;[0 0.3125 0.09095] Set roles
  (CallFunction|GivePlayerRoles (Variables|Default|GetRolePool))
  (CallFunction|GiveKillerRoles 1))

(event Custom|ResetPlayers
  (bind _housesarray (Variables|Default|GetHousesArray))
  ;[0.6029 0 1] Reset players
  (CallFunction|GenerateHouses _housesarray)
  (Utilities|FlowControl|Delay 0.2)
  (for _array_element (CallFunction|PCArray)
    (CallFunction|SpawnPlayer _array_element)
    (Development|PrintString (Utilities|String|Append (Utilities|GetDisplayName _array_element) " " (Utilities|GetDisplayName (.Value (Utilities|Map|Find _housesarray _array_element)))))
    (Default|RemoveLoadingScreenAfter _array_element 1.0)
    (Utilities|FlowControl|Delay 1.0)
    (bind _asgs_game (Utilities|Casting|CastToGS_Game (Game|GetGameState)))
    (Variables|/Game/_Main/Game/GS_Game.GS_Game_C|SetHasGameStarted _asgs_game true)))

(event Custom|StartDayNightCycle)

(event Custom|EndGame
  (params (VillageWin :type Boolean))
  (for _array_element (Variables|/Script/Engine.GameStateBase|GetPlayerArray (Game|GetGameState))
    (bind _aspc_game (Utilities|Casting|CastToPC_Game (Game|GetPlayerController _array_element)))
    (Default|PlayerEndGame _aspc_game VillageWin)))

(event EventBeginPlay
  (if (not (Variables|Default|GetInDebug))
    (Utilities|FlowControl|Delay 3.0)
    (CallFunction|SetPlayersRoles)
    (CallFunction|ResetPlayers)
    (Default|CallSetDayTime 6.0)))

(event EventTick
  (params (DeltaSeconds :type Float%20%28single-precision%29)))

(event EventPostLogin
  (params (NewPlayer :type Player%20Controller%20Object%20Reference))
  ;[1 0 0.5838] When a player join
  (if (not (Variables|Default|GetInDebug))
    (bind _aspc_game (Utilities|Casting|CastToPC_Game NewPlayer))
    (Default|ShowLoadingScreen _aspc_game)))

(fn ConstructionScript)

(fn FindPlayerStart
  (params (Player :type Controller%20Object%20Reference) (IncomingName :type String))
  (bind _outactors (Actor|GetAllActorsOfClass "/Script/Engine.PlayerStart"))
  (for _array_element _outactors
    (bind _aspc_game (Utilities|Casting|CastToPC_Game Player))
    (if (Utilities|Enum|Equal(Enum) (Utilities|String|ToString(Name) (Variables|/Script/Engine.PlayerStart|GetPlayerStartTag _array_element)) (Utilities|String|EnumtoString (Variables|/Game/_Main/Game/PC_Game.PC_Game_C|GetPlayerRole _aspc_game)))
      (return _array_element)
      (elif (Utilities|Enum|Equal(Enum) (Utilities|String|ToString(Name) (Variables|/Script/Engine.PlayerStart|GetPlayerStartTag _array_element)) "default")
        (LocalVariables|SetDefaultSpawn _array_element))))
  (bind _defaultspawn (LocalVariables|GetDefaultSpawn)
    (:then
      (return _defaultspawn))
    (:else)))

(fn SpawnPlayer
  (params (PC :type PC%20Game%20Object%20Reference))
  (bind _housesarray (Variables|Default|GetHousesArray))
  (bind _returnvalue (Game|GetInstigator PC))
  (bind (_value _returnvalue_2) (Utilities|Map|Find _housesarray PC))
  (|Destroycharacterifownone
    (:OutputPin
      (if _returnvalue_2
        (Utilities|IsValid _value
          (:Is%20Valid
            (bind _returnvalue_3 (Game|SpawnActorfromClass "/Game/_Main/Game/Characters/PCC_Game.PCC_Game_C" (Default|PlayerSpawnTransform _value) "Undefined" 0 _returnvalue))
            (Pawn|Possess PC _returnvalue_3)
            (Default|OnCharacterSpawnin _value _returnvalue_3))
          (:Is%20Not%20Valid
            ;[0 0.2839 1] If this PC doesnt have a house
            (bind _returnvalue_4 (Game|SpawnActorfromClass "/Game/_Main/Game/Characters/PCC_Game.PCC_Game_C" (Transformation|GetActorTransform (Class|GameModeBase|FindPlayerStart PC)) "Undefined" 0 _returnvalue :!label _label))
            (Pawn|Possess PC _returnvalue_4)))
        (else
          (goto _label))))))

(fn ShufflePCList
  (Utilities|Array|Clear (LocalVariables|GetPCList))
  (for _array_element (Variables|/Script/Engine.GameStateBase|GetPlayerArray (Game|GetGameState))
    (bind _aspc_game (Utilities|Casting|CastToPC_Game (Game|GetPlayerController _array_element)))
    (Utilities|Array|AddUnique (LocalVariables|GetPCList) _aspc_game))
  (Utilities|Array|Shuffle (LocalVariables|GetPCList))
  (return (LocalVariables|GetPCList)))

(fn PCArray
  (for _array_element (Variables|/Script/Engine.GameStateBase|GetPlayerArray (Game|GetGameState))
    (bind _aspc_game (Utilities|Casting|CastToPC_Game (Game|GetPlayerController _array_element)))
    (Utilities|Array|Add (LocalVariables|GetPCList) _aspc_game))
  (return (LocalVariables|GetPCList)))

(fn GetHouseSpawnpointatIndex
  (params (At%20index :type Integer))
  (bind _outactors (Actor|GetAllActorsOfClass "/Game/_Main/Game/Blueprints/BP_HouseSpawnpoint.BP_HouseSpawnpoint_C"))
  (for _array_element _outactors
    (if (== (Variables|/Game/_Main/Game/Blueprints/BP_HouseSpawnpoint.BP_HouseSpawnpoint_C|GetIndex _array_element) At%20index)
      (return true _array_element)))
  (return false 0))

(fn SpawnHouseatIndex
  (params (At%20index :type Integer) (Role :type ERole%20Enum :default "NewEnumerator0"))
  (bind (_found _spawnpoint) (CallFunction|GetHouseSpawnpointatIndex At%20index))
  (if _found
    (bind _asbp_house (Utilities|Casting|CastToBP_HouseClass (Utilities|Select :Index Role :NewEnumerator0 "/Game/_Main/Game/Blueprints/Houses/BP_House_Hunter.BP_House_Hunter_C" :NewEnumerator1 "/Game/_Main/Game/Blueprints/Houses/BP_House_Witch.BP_House_Witch_C" :NewEnumerator2 "/Game/_Main/Game/Blueprints/Houses/BP_House_Farmer.BP_House_Farmer_C" :NewEnumerator3 "/Game/_Main/Game/Blueprints/Houses/BP_House_Incantatrice.BP_House_Incantatrice_C")))
    (bind _returnvalue (Game|SpawnActorfromClass _asbp_house (Transformation|GetActorTransform _spawnpoint) "AlwaysSpawn" 0 0))
    (Default|OnSpawned _returnvalue At%20index)
    (return _returnvalue)
    (else
      (Development|PrintString "Error: no spawnpoint found for a house" true true "(R=1.000000,G=0.000000,B=0.000000,A=1.000000)" 5e+01))))

(fn GenerateHouses
  (params (TargetMap :type Map%20of%20Player%20Controller%20Object%20References%20to%20Objects))
  (CallFunction|CleanSpawnedHouses TargetMap)
  (bind _output_get (LocalVariables|SetShuffledPlayerListLocal (CallFunction|ShufflePCList)))
  (for (_array_element _array_index) _output_get
    (bind _house_spawned (CallFunction|SpawnHouseatIndex _array_index (Variables|/Game/_Main/Game/PC_Game.PC_Game_C|GetPlayerRole _array_element)))
    (Default|OnOwnedbyPC _house_spawned _array_element)
    (Utilities|Map|Add TargetMap _array_element _house_spawned)
    (Development|PrintString (Utilities|String|Append "Added  " (Utilities|GetDisplayName _array_element) " " (Utilities|GetDisplayName _house_spawned))))
  (return TargetMap))

(fn CleanSpawnedHouses
  (params (HousesArray :type Map%20of%20Player%20Controller%20Object%20References%20to%20Objects))
  (bind _values (Utilities|Map|Values HousesArray))
  (for _array_element _values
    (Utilities|IsValid _array_element
      (:Is%20Valid
        (Default|CleanHouse _array_element)
        (Actor|DestroyActor _array_element))
      (:Is%20Not%20Valid
        (Development|PrintString "HouseNotValid" true true "(R=1.000000,G=0.000000,B=0.000000,A=1.000000)"))))
  (Utilities|Map|Clear HousesArray))

(fn GivePlayerRoles
  (params (RolesPool :type Array%20of%20ERole%20Enums :default "NewEnumerator0"))
  (LocalVariables|SetRolePoleLocal RolesPool)
  (for _array_element (Variables|/Script/Engine.GameStateBase|GetPlayerArray (Game|GetGameState))
    (bind _aspc_game (Utilities|Casting|CastToPC_Game (Game|GetPlayerController _array_element)))
    (bind _output_get (LocalVariables|SetChosenRole (.OutItem (Utilities|Array|Random (LocalVariables|GetRolePoleLocal)))))
    (Utilities|Array|RemoveIndex (LocalVariables|GetRolePoleLocal) (Utilities|Array|FindItem (LocalVariables|GetRolePoleLocal) _output_get))
    (Variables|/Game/_Main/Game/PC_Game.PC_Game_C|SetPlayerRole _aspc_game (LocalVariables|GetChosenRole))))

(fn GiveKillerRoles
  (params (NB :type Integer))
  (Utilities|Array|Clear (LocalVariables|GetPendingPlayers))
  (for _array_element (Variables|/Script/Engine.GameStateBase|GetPlayerArray (Game|GetGameState))
    (bind _aspc_game (Utilities|Casting|CastToPC_Game (Game|GetPlayerController _array_element)))
    (Variables|/Game/_Main/Game/PC_Game.PC_Game_C|SetIsTheKiller _aspc_game false)
    (Utilities|Array|AddUnique (LocalVariables|GetPendingPlayers) _aspc_game))
  (Utilities|Array|Shuffle (LocalVariables|GetPendingPlayers))
  (for _index (range 0 (- NB 1))
    (Variables|/Game/_Main/Game/PC_Game.PC_Game_C|SetIsTheKiller (Utilities|Array|Get(acopy) (LocalVariables|GetPendingPlayers) _index) true)))