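; Skybox actor that switches the level between day and night looks.
; SetTime stores the Day flag, then swaps the sky mesh material and adjusts the sky light and two directional lights' intensities, plus the directional lights' colors.
; The construction script applies the current Day setting.
; On authority only, Tick runs through a Delay to call the server time-change event, flipping Day roughly every ten seconds.
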(event Custom|ChangeTime_Server
  (CallFunction|SetTime (not (Variables|Default|GetDay?))))

(event EventBeginPlay)

(event Collision|EventActorBeginOverlap
  (params (OtherActor :type Actor%20Object%20Reference)))

(event EventTick
  (params (DeltaSeconds :type Float%20%28single-precision%29))
  (Networking|SwitchHasAuthority
    (:Authority
      (Utilities|FlowControl|Delay 1e+01)
      (CallFunction|ChangeTimeServer))))

(fn ConstructionScript
  (CallFunction|SetTime (Variables|Default|GetDay?)))

(fn SetTime
  (params (isDay :type Boolean))
  (bind _skylight (Variables|Default|GetSkyLight))
  (bind _directionallight (Variables|Default|GetDirectionalLight))
  (bind _directionallight1 (Variables|Default|GetDirectionalLight1))
  (Variables|Default|SetDay? isDay)
  (if (Variables|Default|GetDay?)
    (Rendering|Material|SetMaterial (Variables|Default|GetStaticMesh) 0 "/Game/Fantastic_Village_Pack/materials/MI_skybox_day.MI_skybox_day")
    (Rendering|Components|Light|SetIntensity _skylight 1.3)
    (Rendering|Components|Light|SetIntensity _directionallight1 3.0)
    (Rendering|Components|Light|SetLightColor _directionallight1 "(R=1.000000,G=0.806952,B=0.205079,A=1.000000)" true)
    (Rendering|Components|Light|SetIntensity _directionallight 12.0)
    (Rendering|Components|Light|SetLightColor _directionallight "(R=1.000000,G=0.806952,B=0.205079,A=1.000000)" true)
    (else
      (Rendering|Material|SetMaterial (Variables|Default|GetStaticMesh) 0 "/Game/Fantastic_Village_Pack/materials/MI_skybox_night.MI_skybox_night")
      (Rendering|Components|Light|SetIntensity _skylight 0.5)
      (Rendering|Components|Light|SetIntensity _directionallight1 0.1)
      (Rendering|Components|Light|SetLightColor _directionallight1 "(R=0.324110,G=0.361988,B=0.536458,A=1.000000)" true)
      (Rendering|Components|Light|SetIntensity _directionallight 0.5)
      (Rendering|Components|Light|SetLightColor _directionallight "(R=0.217936,G=0.274753,B=0.536458,A=1.000000)" true))))