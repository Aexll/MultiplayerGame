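; Lobby game mode that tracks connected players and keeps each one's player list up to date.
; PostLogin adds the new controller to Players and logout removes the exiting PC_Lobby, then both run the shared NewPlayer event.
; NewPlayer rebuilds PlayersNames from each PC_Lobby's Name, then passes the full list to every controller through SetPlayerList.
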(event Custom|NewPlayer
  (Utilities|Array|Clear (Variables|Default|GetPlayersNames))
  (for _array_element (Variables|Default|GetPlayers)
    (bind _aspc_lobby (Utilities|Casting|CastToPC_Lobby _array_element))
    (Utilities|Array|Add (Variables|Default|GetPlayersNames) (Variables|/Game/Main/Lobby/PC_Lobby.PC_Lobby_C|GetName _aspc_lobby)))
  (for _array_element_2 (Variables|Default|GetPlayers)
    (bind _aspc_lobby_2 (Utilities|Casting|CastToPC_Lobby _array_element_2))
    (Default|SetPlayerList _aspc_lobby_2 (Variables|Default|GetPlayersNames))))

(event EventBeginPlay)

(event EventTick
  (params (DeltaSeconds :type Float%20%28single-precision%29)))

(event EventPostLogin
  (params (NewPlayer :type Player%20Controller%20Object%20Reference))
  (Utilities|Array|AddUnique (Variables|Default|GetPlayers) NewPlayer)
  (CallFunction|NewPlayer))

(event EventOnLogout
  (params (ExitingController :type Controller%20Object%20Reference))
  (bind _aspc_lobby (Utilities|Casting|CastToPC_Lobby ExitingController))
  (Utilities|Array|RemoveItem (Variables|Default|GetPlayers) _aspc_lobby)
  (CallFunction|NewPlayer))

(fn ConstructionScript)