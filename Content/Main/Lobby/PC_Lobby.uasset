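; Lobby player controller that shows the list of players on the lobby HUD.
; On BeginPlay, a client event copies the player name from the GI game instance into the controller.
; Player list updates are forwarded to a client event, which passes them to the Widget_Lobby HUD.
; WidgetValidator lazily creates that widget and keeps it in the viewport before each update.
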(event Custom|SetPlayerList_Client
  (params (PlayerList :type Array%20of%20Strings))
  ;[1 0.3333 0] Comment
  (Utilities|WidgetValidator)
  (Default|SetPlayers (Variables|Default|GetHUD) PlayerList))

(event Custom|BeginPlay_Client
  ;[1 0.3333 0] Comment
  (bind _asgi (Utilities|Casting|CastToGI (Game|GetGameInstance)))
  (Variables|Default|SetName (Variables|/Game/Main/GI.GI_C|GetPlayerName _asgi)))

(event Custom|SetPlayerList
  (params (PlayerList :type Array%20of%20Strings))
  ;[0 0.3333 1] Comment
  (CallFunction|SetPlayerListClient PlayerList))

(event EventBeginPlay
  (CallFunction|BeginPlayClient))

(event EventTick
  (params (DeltaSeconds :type Float%20%28single-precision%29)))

(fn ConstructionScript)