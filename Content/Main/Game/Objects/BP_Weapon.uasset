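; BP_Weapon is a melee weapon that, when used, plays a slash swing and hits what the user aims at, gated by a short cooldown.
; The server use event multicasts a timeline that rotates the mesh from its current relative rotation.
; It also line traces from the user's camera along control rotation, applying hit damage and pushing physics-simulating components, with debug drawing left on.
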(event Custom|Used_Multicast
  (params (Relative%20Rotation :type Rotator))
  (bind _newtrack_0 (Timeline|Slash PlayFromStart)
    (:Update
      (Transformation|SetRelativeRotation (Variables|Default|GetStaticMesh) (Math|Rotator|CombineRotators Relative%20Rotation (Math|Rotator|Lerp(Rotator) "0,0.000000, 0" "-90.000000,-20.000000,0.000000" _newtrack_0)) false false))))

(event EventBeginPlay
  (|CallParentFunction))

(event Collision|EventActorBeginOverlap
  (params (OtherActor :type Actor%20Object%20Reference)))

(event EventTick
  (params (DeltaSeconds :type Float%20%28single-precision%29))
  (|CallParentFunction DeltaSeconds) ; This node is disabled and will not be called.\nDrag off pins to build functionality.
)

(event EventUsedServer
  (params (By :type PCC%20Game%20Object%20Reference))
  (bind _camera (Variables|/Game/Main/Game/PCC_Game.PCC_Game_C|GetCamera By))
  (bind _returnvalue (Transformation|GetWorldLocation _camera))
  (Utilities|Cooldown 0.5
    (:then_0
      (CallFunction|UsedMulticast (Variables|/Script/Engine.SceneComponent|GetRelativeRotation (Variables|Default|GetStaticMesh)))
      (Utilities|IsValid By
        (:Is%20Valid
          (bind (_outhit _returnvalue_2) (Collision|LineTraceByChannel _returnvalue (+ _returnvalue (* (Math|Vector|GetForwardVector (Pawn|GetControlRotation By :!class /Script/Engine.Pawn)) (Variables|Default|GetRange))) "TraceTypeQuery1" false (Utilities|Array|MakeArray By) "ForDuration"))
          (if _returnvalue_2
            (Game|Damage|ApplyDamage (.HitActor (Collision|BreakHitResult _outhit)) (Variables|Default|GetDamages) 0 0 "/Game/Main/Game/DamageSystem/DMG_Hit.DMG_Hit_C")
            (Utilities|IsValid (.HitComponent (Collision|BreakHitResult _outhit))
              (:Is%20Valid
                (if (Physics|IsSimulatingPhysics (.HitComponent (Collision|BreakHitResult _outhit)) (.HitBoneName (Collision|BreakHitResult _outhit)))
                  (Physics|AddImpulseatLocation (.HitComponent (Collision|BreakHitResult _outhit)) (* (.ImpactNormal (Collision|BreakHitResult _outhit)) -10000) (.ImpactPoint (Collision|BreakHitResult _outhit)) (.HitBoneName (Collision|BreakHitResult _outhit))))))))))))

(fn ConstructionScript
  (|CallParentFunction))