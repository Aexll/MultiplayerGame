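; Grabbable gun object that fires a hitscan shot when used, and also goes off when it takes fire damage.
; The server rate-limits shots with a cooldown macro, tracing from the user's camera or, without a user, from the gun's mesh.
; Hits receive damage and push simulating physics components, while a multicast plays the shot sound and Niagara effect.
; Fire damage also randomizes the shot cooldown.
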(event Custom|Used_Multicast
  (params (ImpactPoint :type Vector))
  (bind _staticmesh (Variables|Default|GetStaticMesh))
  (bind _returnvalue (Transformation|GetSocketTransform _staticmesh "Fire" "RTS_World"))
  (bind (_location _rotation) (Math|Transform|BreakTransform _returnvalue))
  ;[1 0.3489 0] Used on all clients
  (if (Transformation|DoesSocketExist _staticmesh "Fire")
    (Audio|PlaySoundatLocation "/Game/Assets/SoundsWAV/Gunshort.Gunshort" _location _rotation 1.0 1.0 0.0 "/Game/Main/Game/Audios/SA_Basic.SA_Basic" 0 0 0)
    (Components|Activation|Activate (Variables|Default|GetNiagara) true)))

(event Custom|OnTakeAnyDamage_Event_1
  (params (DamagedActor :type Actor%20Object%20Reference) (Damage :type Float%20%28single-precision%29) (DamageType :type Damage%20Type%20Object%20Reference) (InstigatedBy :type Controller%20Object%20Reference) (DamageCauser :type Actor%20Object%20Reference))
  ;[1 0.06395 0] When taking fire damages
  (Utilities|Casting|CastToDMG_Fire DamageType)
  (CallFunction|UsedServer)
  (Variables|Default|SetShoutCooldown (+ (* (Math|Random|RandomFloat) 5.0) 1.0)))

(event EventBeginPlay
  (|CallParentFunction)
  ;[1 0.06395 0] When taking fire damages
  (EventDispatchers|AssignOnTakeAnyDamage (delegate Custom|OnTakeAnyDamage_Event_1)))

(event Collision|EventActorBeginOverlap
  (params (OtherActor :type Actor%20Object%20Reference)))

(event EventTick
  (params (DeltaSeconds :type Float%20%28single-precision%29))
  (|CallParentFunction DeltaSeconds) ; This node is disabled and will not be called.\nDrag off pins to build functionality.
)

(event EventUsedServer
  (params (By :type PCC%20Game%20Object%20Reference))
  (bind _graber (Variables|Default|GetGraber))
  ;[0.04239 0 1] When used (on server)
  (Utilities|Coodlownize (Variables|Default|GetShoutCooldown)
    (:Out
      (bind _outhit (CallFunction|GetShoutOuputHit By))
      (CallFunction|UsedMulticast (.ImpactPoint (Collision|BreakHitResult _outhit)))
      (Utilities|IsValid (.HitComponent (Collision|BreakHitResult _outhit))
        (:Is%20Valid
          (if (Physics|IsSimulatingPhysics (.HitComponent (Collision|BreakHitResult _outhit)) (.HitBoneName (Collision|BreakHitResult _outhit)))
            (Physics|AddImpulseatLocation (.HitComponent (Collision|BreakHitResult _outhit)) (* (.ImpactNormal (Collision|BreakHitResult _outhit)) -10000) (.ImpactPoint (Collision|BreakHitResult _outhit)) (.HitBoneName (Collision|BreakHitResult _outhit))))
          (Game|Damage|ApplyDamage (.HitActor (Collision|BreakHitResult _outhit)) 1.0 0 (select (Utilities|IsValid _graber) _graber self) "/Game/Main/Game/DamageSystem/DMG_Hit.DMG_Hit_C"))))))

(fn ConstructionScript
  (|CallParentFunction))

(fn GetShoutOuputHit
  (params (User :type PCC%20Game%20Object%20Reference))
  (bind _range (Variables|Default|GetRange))
  (bind _camera (Variables|/Game/Main/Game/PCC_Game.PCC_Game_C|GetCamera User))
  (bind _staticmesh (Variables|Default|GetStaticMesh))
  (bind _returnvalue (Transformation|GetWorldLocation _camera))
  (bind _returnvalue_2 (Transformation|GetSocketTransform _staticmesh "None" "RTS_World"))
  (bind (_location _rotation) (Math|Transform|BreakTransform _returnvalue_2))
  (Utilities|IsValid User
    (:Is%20Valid
      (bind _outhit (Collision|LineTraceByChannel _returnvalue (+ _returnvalue (* (Math|Vector|GetForwardVector (Pawn|GetControlRotation User :!class /Script/Engine.Pawn)) _range)) "TraceTypeQuery1" false (Utilities|Array|MakeArray User) "ForDuration"))
      (return _outhit))
    (:Is%20Not%20Valid
      (if (Transformation|DoesSocketExist _staticmesh "Fire")
        (bind _outhit_2 (Collision|LineTraceByChannel _location (+ (* (Math|Vector|GetForwardVector _rotation) _range) _location) "TraceTypeQuery1" false 0 "ForDuration"))
        (return _outhit_2)
        (else
          (Development|PrintString "Error this gun needs a socket" true true "(R=1.000000,G=0.000000,B=0.000000,A=1.000000)"))))))