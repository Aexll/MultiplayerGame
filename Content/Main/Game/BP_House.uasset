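; BP_House is a house that provides a player spawn transform and has a door keyed to its index.
; On spawn it stores the given index and copies it to the BP_Door child actor's KeyIndex.
; When a character spawns in, it adds that index to the character's Keys without duplicates.
; PlayerSpawnTransform returns the TempSpawnpoint's world transform, while the ownership and cleanup events are empty stubs.
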(event Custom|OnOwnedByPC
  (params (PC :type PC%20Object%20Reference)))

(event Custom|OnCharacterSpawnIn
  (params (PCC :type PCC%20Game%20Object%20Reference))
  (Utilities|Array|AddUnique (Variables|/Game/Main/Game/PCC_Game.PCC_Game_C|GetKeys PCC) (Variables|Default|GetHouseIndex)))

(event Custom|CleanHouse)

(event Custom|OnSpawned
  (params (MyIndex :type Integer))
  (Variables|Default|SetHouseIndex MyIndex)
  (bind _asbp_door (Utilities|Casting|CastToBP_Door (Variables|/Script/Engine.ChildActorComponent|GetChildActor (Variables|Default|GetBP_Door))))
  (Variables|/Game/Main/Game/BP_Door.BP_Door_C|SetKeyIndex _asbp_door (Variables|Default|GetHouseIndex)))

(event EventBeginPlay)

(event Collision|EventActorBeginOverlap
  (params (OtherActor :type Actor%20Object%20Reference)))

(event EventTick
  (params (DeltaSeconds :type Float%20%28single-precision%29)))

(fn ConstructionScript)

(fn PlayerSpawnTransform
  (return (Transformation|GetWorldTransform (Variables|Default|GetTempSpawnpoint))))