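; Actor component that tracks the owner's temperature and applies cold or fire damage when it leaves the safe range.
; On authority-only Tick, temperature eases toward the last entry in Boxes, or the GameState ambient (with hardcoded fallback), at that source's diffusion rate.
; Damage scales with distance beyond the thresholds while temperature is changing.
; A Client event receives each update and, for PCC_Game owners, drives Freeze and Fire parameters in a material parameter collection.
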(event Custom|Client
  (params (InDouble :type Float%20%28double-precision%29))
  (bind _output_get (Variables|Default|SetTemperature InDouble))
  (Utilities|Casting|CastToPCC_Game (Components|GetOwner))
  (Rendering|Material|SetScalarParameterValue "/Game/Main/Game/PostProcess/MPC_Testing.MPC_Testing" "Freeze" (Math|Float|Clamp(Float) (* (- 5.0 _output_get) 0.1)) :!class /Script/Engine.KismetMaterialLibrary)
  (Rendering|Material|SetScalarParameterValue "/Game/Main/Game/PostProcess/MPC_Testing.MPC_Testing" "Fire" (Math|Float|Clamp(Float) (* (- (Variables|Default|GetTemperature) 5e+01) 0.1)) :!class /Script/Engine.KismetMaterialLibrary))

(event EventBeginPlay
  (Components|Tick|SetComponentTickEnabled (Ability|HasAuthority (Components|GetOwner)))
  (Variables|Default|SetTemperature (.AmbianteTemperature (CallFunction|GetAmbianteTemperature))))

(event EventTick
  (params (DeltaSeconds :type Float%20%28single-precision%29))
  (bind _returnvalue (Components|GetOwner))
  (bind (_ambiantetemperature _ambiantdiffusion) (CallFunction|GetAmbianteTemperature))
  (bind _boxes (Variables|Default|GetBoxes))
  (bind _returnvalue_2 (Utilities|Array|LastIndex _boxes))
  (bind _output (Utilities|Array|Get(acopy) _boxes _returnvalue_2))
  (Utilities|IsValid _output
    (:Is%20Valid
      (Variables|Default|SetTargetTemperature (Variables|/Game/Main/Game/BP_Field.BP_Field_C|GetTemperature _output))
      (Variables|Default|SetTargetDiffusion (Variables|/Game/Main/Game/BP_Field.BP_Field_C|GetDiffusion _output)))
    (:Is%20Not%20Valid
      (Variables|Default|SetTargetTemperature _ambiantetemperature)
      (Variables|Default|SetTargetDiffusion _ambiantdiffusion)))
  (if (!= (Variables|Default|GetTemperature) (Variables|Default|GetTargetTemperature))
    (bind _output_get (Variables|Default|SetTemperature (CallFunction|LerpTillTresshold (Variables|Default|GetTemperature) (Variables|Default|GetTargetTemperature) (/ (Variables|Default|GetTargetDiffusion) 1e+02) 0.1)))
    (CallFunction|Client _output_get)
    (if (< _output_get 0.0)
      (Game|Damage|ApplyDamage _returnvalue (/ (Variables|Default|GetTemperature) -1e+03) 0 0 "/Game/Main/Game/DamageSystem/DMG_Cold.DMG_Cold_C")
      (elif (> _output_get 5e+01)
        (Game|Damage|ApplyDamage _returnvalue (/ (- (Variables|Default|GetTemperature) 5e+01) 1e+03) 0 0 "/Game/Main/Game/DamageSystem/DMG_Fire.DMG_Fire_C")))))

(fn GetAmbianteTemperature
  (Utilities|IsValid (Variables|World|GetGS)
    (:Is%20Valid
      _)
    (:Is%20Not%20Valid
      (bind _asgs (Utilities|Casting|CastToGS (Game|GetGameState))
        (:then
          (Variables|World|SetGS _asgs))
        (:CastFailed
          (return 19.0 0.5)))))
  (return (Variables|/Game/Main/Game/GS.GS_C|GetAmbianteTemperature (Variables|World|GetGS)) (Variables|/Game/Main/Game/GS.GS_C|GetAmbiantDiffusion (Variables|World|GetGS))))