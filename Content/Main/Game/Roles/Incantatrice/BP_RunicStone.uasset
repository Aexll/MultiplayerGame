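; Runic stone actor for the Incantatrice role that shows an indexed rune and breaks when it takes any damage.
; Damage is bound on the authority only, where breaking multicasts a particle burst and lightning sound, then destroys the stone.
; Its material receives the stone index on BeginPlay, and an excitement timeline ("Exitment") drives the Force parameter, playing forward or reversing through start and stop events.
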(event Custom|SetStoneIndex
  (params (Index :type Integer))
  (Rendering|Material|SetScalarParameterValue (Variables|Default|GetMaterial) "Index" (Math|Conversions|ToFloat(Integer) Index) :!class /Script/Engine.MaterialInstanceDynamic))

(event Custom|StartExited
  (bind _newtrack_0 (Timeline|Exitment Play)
    (:Update
      (CallFunction|SetExited _newtrack_0))))

(event Custom|StopExited
  (bind _newtrack_0 (Timeline|Exitment Reverse)
    (:Update
      (CallFunction|SetExited _newtrack_0))))

(event Custom|OnDamaged
  (params (DamagedActor :type Actor%20Object%20Reference) (Damage :type Float%20%28single-precision%29) (DamageType :type Damage%20Type%20Object%20Reference) (InstigatedBy :type Controller%20Object%20Reference) (DamageCauser :type Actor%20Object%20Reference))
  (CallFunction|BreakStoneServer))

(event Custom|BreakStone_Server
  (CallFunction|BreakStoneMulticast)
  (CallFunction|DestroyServer))

(event Custom|BreakStone_Multicast
  (bind _staticmesh (Variables|Default|GetStaticMesh))
  (bind _returnvalue (Transformation|GetWorldTransform _staticmesh))
  (Niagara|SpawnSystematLocation "/Game/Main/Game/Roles/Incantatrice/P_RuneBreak.P_RuneBreak" (.location _returnvalue) (.rotation _returnvalue) (.scale _returnvalue))
  (Audio|PlaySoundatLocation "/Game/Magic___Spell_Sounds_PRO/Elements___School/Lightning/cue/Lightning_Spell_8_Cue.Lightning_Spell_8_Cue" (.location _returnvalue) "0, 0, 0" 1.0 1.0 0.0 "/Game/Main/Game/Audios/SA_Basic.SA_Basic" 0 0 0))

(event Custom|SetExited
  (params (Exitement :type Float%20%28double-precision%29))
  (Rendering|Material|SetScalarParameterValue (Variables|Default|GetMaterial) "Force" Exitement :!class /Script/Engine.MaterialInstanceDynamic))

(event EventBeginPlay
  (|CallParentFunction)
  (CallFunction|SetStoneIndex (Variables|ServerOnly|GetStoneIndex))
  (Networking|SwitchHasAuthority
    (:Authority
      (EventDispatchers|BindEventtoOnTakeAnyDamage (delegate Custom|OnDamaged)))))

(event Collision|EventActorBeginOverlap
  (params (OtherActor :type Actor%20Object%20Reference)))

(event EventTick
  (params (DeltaSeconds :type Float%20%28single-precision%29))
  (|CallParentFunction DeltaSeconds) ; This node is disabled and will not be called.\nDrag off pins to build functionality.
)

(fn ConstructionScript
  (|CallParentFunction))