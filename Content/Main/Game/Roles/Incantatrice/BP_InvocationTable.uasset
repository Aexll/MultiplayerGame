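; Invocation table for the Incantatrice role that performs a ritual when a runic scroll and enough runic stones lie in its box.
; Server-only overlaps track scroll and stones, checking the count against the scroll's Incantation class defaults.
; A timeline turns off their gravity and drives one Force value for rune glow, particles, sound and radial force, reversing quickly if requirements break.
; On completion it breaks the required stones and invokes the scroll.
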(event OnComponentBeginOverlap(Box)
  (params (OverlappedComponent :type Primitive%20Component%20Object%20Reference) (OtherActor :type Actor%20Object%20Reference) (OtherComp :type Primitive%20Component%20Object%20Reference) (OtherBodyIndex :type Integer) (bFromSweep :type Boolean) (SweepResult :type Hit%20Result%20Structure%20%28by%20ref%29))
  (Networking|SwitchHasAuthority
    (:Authority
      (Utilities|FlowControl|Sequence
        (:then_0
          (bind _asbp_runic_scroll (Utilities|Casting|CastToBP_RunicScroll OtherActor)
            (:then
              (Utilities|IsValid (Variables|ServerOnly|GetCurrentParchemin)
                (:Is%20Not%20Valid
                  (CallFunction|ScrollTrigger _asbp_runic_scroll true)
                  (Variables|ServerOnly|SetCurrentParchemin _asbp_runic_scroll))))
            (:CastFailed
              (bind _asbp_runic_stone (Utilities|Casting|CastToBP_RunicStone OtherActor))
              (CallFunction|StoneTrigger _asbp_runic_stone true)
              (Utilities|Array|AddUnique (Variables|Default|GetAviableStones) _asbp_runic_stone))))
        (:then_1
          (if (CallFunction|IsReadytoInvoke)
            (CallFunction|StartRituel)))))))

(event OnComponentEndOverlap(Box)
  (params (OverlappedComponent :type Primitive%20Component%20Object%20Reference) (OtherActor :type Actor%20Object%20Reference) (OtherComp :type Primitive%20Component%20Object%20Reference) (OtherBodyIndex :type Integer))
  (bind _box (Variables|Default|GetBox))
  (bind _overlappingactors (Collision|GetOverlappingActors _box "/Game/Main/Game/Roles/Incantatrice/BP_RunicScroll.BP_RunicScroll_C" :!class /Script/Engine.PrimitiveComponent))
  (Networking|SwitchHasAuthority
    (:Authority
      (Utilities|FlowControl|Sequence
        (:then_0
          (bind _asbp_runic_scroll (Utilities|Casting|CastToBP_RunicScroll OtherActor)
            (:then
              (CallFunction|ScrollTrigger _asbp_runic_scroll false)
              (if (== (Utilities|Array|Length _overlappingactors) 1)
                (bind _asbp_runic_scroll_2 (Utilities|Casting|CastToBP_RunicScroll (Utilities|Array|Get(acopy) _overlappingactors)))
                (CallFunction|FocusScroll _asbp_runic_scroll_2)
                (else
                  (Variables|ServerOnly|SetCurrentParchemin 0)
                  (CallFunction|UnFocus))))
            (:CastFailed
              (bind _asbp_runic_stone (Utilities|Casting|CastToBP_RunicStone OtherActor))
              (CallFunction|StoneTrigger _asbp_runic_stone false)
              (Utilities|Array|RemoveItem (Variables|Default|GetAviableStones) _asbp_runic_stone))))
        (:then_1
          (if (not (CallFunction|IsReadytoInvoke))
            (CallFunction|StopRituel)))))))

(event Custom|SetForce
  (params (Force :type Float%20%28double-precision%29))
  (bind _mat1 (Variables|Default|GetMat1))
  (Rendering|Material|SetScalarParameterValue _mat1 "Emissive Intensity" (Math|Float|Lerp 0.0 2e+01 Force) :!class /Script/Engine.MaterialInstanceDynamic)
  (Rendering|Material|SetVectorParameterValue _mat1 "Emissive Color" (Math|Color|Lerp(LinearColor) "(R=0.479167,G=0.479167,B=0.479167,A=1.000000)" (Variables|Default|GetCurrentColor) (* Force 4.0)) :!class /Script/Engine.MaterialInstanceDynamic)
  (Effects|Components|ParticleSystem|SetFloatParameter (Variables|Default|GetP_RuneAttraction) "Force" Force)
  (Audio|Components|Audio|SetVolumeMultiplier (Variables|Default|GetPad_Loop_04_Cue) Force :!class /Script/Engine.AudioComponent)
  (Variables|/Script/Engine.RadialForceComponent|SetForceStrength (Variables|Default|GetRadialForce) (Math|Float|Lerp -8e+02 0.0 Force)))

(event Custom|UnFocus
  ;[0.08164 0 1] Focus Scroll
  (Components|Timeline|SetPlayRate (Variables|Default|GetInvokeTimeline) 1e+01)
  (bind _currentparchemin (Variables|ServerOnly|GetCurrentParchemin)
    (:then
      (CallFunction|ScrollTrigger _currentparchemin false))
    (:else)))

(event Custom|FocusScroll
  (params (Scroll :type BP%20Runic%20Scroll%20Object%20Reference))
  ;[0.08164 0 1] Focus Scroll
  (Components|Timeline|SetPlayRate (Variables|Default|GetInvokeTimeline) 1.0)
  (bind _output_get (Variables|ServerOnly|SetCurrentParchemin Scroll))
  (CallFunction|ScrollTrigger _output_get true))

(event Custom|StopRituel
  (for _array_element (Variables|Default|GetAviableStones)
    (Default|SetGravityServer _array_element true))
  (bind _currentparchemin (Variables|ServerOnly|GetCurrentParchemin)
    (:then
      (Default|SetGravityServer _currentparchemin true))
    (:else
      _))
  (Components|Timeline|SetPlayRate (Variables|Default|GetInvokeTimeline) 1e+01)
  (bind _newtrack_0 (Timeline|InvokeTimeline Reverse)
    (:Update
      (bind _output_get (Variables|Default|SetForce _newtrack_0))
      (CallFunction|SetForce _output_get)
      (bind _currentparchemin_2 (Variables|ServerOnly|GetCurrentParchemin)
        (:then
          (Transformation|SetActorRotation _currentparchemin_2 (Math|Rotator|Lerp(Rotator) (Transformation|GetActorRotation _currentparchemin_2) (Transformation|GetWorldRotation (Variables|Default|GetMiddlePoint)) 0.01)))
        (:else)))
    (:Finished
      (Components|Timeline|SetNewTime (Variables|Default|GetInvokeTimeline) 0.0)
      (if (CallFunction|IsReadytoInvoke)
        (CallFunction|Invoke)
        (bind _currentparchemin_3 (Variables|ServerOnly|GetCurrentParchemin)
          (:then
            (CallFunction|ScrollTrigger _currentparchemin_3 false)
            (if (CallFunction|IsReadytoInvoke)
              (CallFunction|StartRituel)))
          (:else))))))

(event Custom|StartRituel
  (for _array_element (CallFunction|GettoUseStones)
    (Default|SetGravityServer _array_element false))
  (bind _currentparchemin (Variables|ServerOnly|GetCurrentParchemin)
    (:then
      (Default|SetGravityServer _currentparchemin false)
      (Default|StartExited _currentparchemin))
    (:else
      _))
  (Components|Timeline|SetPlayRate (Variables|Default|GetInvokeTimeline) 1.0)
  (bind _newtrack_0 (Timeline|InvokeTimeline Play)
    (:Update
      (bind _output_get (Variables|Default|SetForce _newtrack_0))
      (CallFunction|SetForce _output_get)
      (bind _currentparchemin_2 (Variables|ServerOnly|GetCurrentParchemin)
        (:then
          (Transformation|SetActorRotation _currentparchemin_2 (Math|Rotator|Lerp(Rotator) (Transformation|GetActorRotation _currentparchemin_2) (Transformation|GetWorldRotation (Variables|Default|GetMiddlePoint)) 0.01)))
        (:else)))
    (:Finished
      (Components|Timeline|SetNewTime (Variables|Default|GetInvokeTimeline) 0.0)
      (if (CallFunction|IsReadytoInvoke)
        (CallFunction|Invoke)
        (bind _currentparchemin_3 (Variables|ServerOnly|GetCurrentParchemin)
          (:then
            (CallFunction|ScrollTrigger _currentparchemin_3 false)
            (if (CallFunction|IsReadytoInvoke)
              (CallFunction|StartRituel)))
          (:else))))))

(event EventBeginPlay
  (Effects|Components|ParticleSystem|SetVectorParameter (Variables|Default|GetP_RuneAttraction) "AttractionPoint" (Transformation|GetWorldLocation (Variables|Default|GetMiddlePoint)))
  (bind _returnvalue (Rendering|Material|CreateDynamicMaterialInstance (Variables|Default|GetStaticMesh) 0 "/Game/DreamscapeSeries/DreamscapeMeadows/Materials/Rocks/MI_RuneRock_01.MI_RuneRock_01" "None" :!class /Script/Engine.PrimitiveComponent))
  (Variables|Default|SetMat1 _returnvalue)
  (bind _returnvalue_2 (Rendering|Material|CreateDynamicMaterialInstance (Variables|Default|GetStaticMesh2) 0 "/Game/DreamscapeSeries/DreamscapeMeadows/Materials/Rocks/MI_RuneRock_02.MI_RuneRock_02" "None" :!class /Script/Engine.PrimitiveComponent))
  (Variables|Default|SetMat2 _returnvalue_2)
  (Rendering|Material|SetMaterial (Variables|Default|GetStaticMesh) 0 (Variables|Default|GetMat1))
  (Rendering|Material|SetMaterial (Variables|Default|GetStaticMesh2) 0 (Variables|Default|GetMat2))
  (CallFunction|SetForce 0.0))

(event Collision|EventActorBeginOverlap
  (params (OtherActor :type Actor%20Object%20Reference)))

(event EventTick
  (params (DeltaSeconds :type Float%20%28single-precision%29)))

(fn ConstructionScript)

(fn ScrollTrigger
  (params (Scroll :type BP%20Runic%20Scroll%20Object%20Reference) (Entering :type Boolean))
  (if Entering
    (Default|SetGravityServer Scroll true)
    (else
      (Default|StopExited Scroll)
      (Default|SetGravityServer Scroll true)))
  (return))

(fn StoneTrigger
  (params (Stone :type BP%20Runic%20Stone%20Object%20Reference) (Enter :type Boolean))
  (if Enter
    (Default|StartExited Stone)
    (else
      (Default|StopExited Stone)))
  (Default|SetGravityServer Stone true)
  (return))

(fn IsReadytoInvoke
  (bind _currentparchemin (Variables|ServerOnly|GetCurrentParchemin)
    (:then
      (return (>= (Utilities|Array|Length (Variables|Default|GetAviableStones)) (Utilities|GetClassDefaults (Variables|/Game/Main/Game/Roles/Incantatrice/BP_RunicScroll.BP_RunicScroll_C|GetIncantation _currentparchemin)))))
    (:else
      (return false))))

(fn Invoke
  (bind _aviablestones (Variables|Default|GetAviableStones))
  (bind _currentparchemin (Variables|ServerOnly|GetCurrentParchemin)
    (:then
      (for _index (range 0 (- (Utilities|GetClassDefaults (Variables|/Game/Main/Game/Roles/Incantatrice/BP_RunicScroll.BP_RunicScroll_C|GetIncantation _currentparchemin)) 1))
        (if (Utilities|Array|IsValidIndex _aviablestones)
          (bind _output_get (LocalVariables|SetConsumeStone (Utilities|Array|Get(acopy) _aviablestones)))
          (Utilities|Array|RemoveIndex _aviablestones)
          (Default|BreakStoneServer _output_get)
          (else
            (return false))))
      (Default|Invoke _currentparchemin)
      (return true))
    (:else
      (return false))))

(fn GettoUseStones
  (bind _aviablestones (Variables|Default|GetAviableStones))
  (bind _currentparchemin (Variables|ServerOnly|GetCurrentParchemin)
    (:then
      (Utilities|Array|Clear (LocalVariables|GetStoness))
      (for _index (range 0 (- (Utilities|GetClassDefaults (Variables|/Game/Main/Game/Roles/Incantatrice/BP_RunicScroll.BP_RunicScroll_C|GetIncantation _currentparchemin)) 1))
        (if (Utilities|Array|IsValidIndex _aviablestones _index)
          (Utilities|Array|AddUnique (LocalVariables|GetStoness) (Utilities|Array|Get(acopy) _aviablestones _index))
          (else
            (return (LocalVariables|GetStoness)))))
      (return (LocalVariables|GetStoness)))
    (:else
      (return 0))))