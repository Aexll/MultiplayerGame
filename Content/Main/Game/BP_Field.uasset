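; BP_Field is a box volume actor that tracks which overlapping actors are inside it through their BPC_Heat component.
; On the server, begin overlap adds the field uniquely to that component's Boxes array and end overlap removes it.
; Begin overlap also prints the other actor's name before the authority check, and the component lookup has no validity check.
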(event OnComponentBeginOverlap(Box)
  (params (OverlappedComponent :type Primitive%20Component%20Object%20Reference) (OtherActor :type Actor%20Object%20Reference) (OtherComp :type Primitive%20Component%20Object%20Reference) (OtherBodyIndex :type Integer) (bFromSweep :type Boolean) (SweepResult :type Hit%20Result%20Structure%20%28by%20ref%29))
  (Development|PrintString (Utilities|GetDisplayName OtherActor))
  (Networking|SwitchHasAuthority
    (:Authority
      (Utilities|Array|AddUnique (Variables|/Game/Main/Game/Components/BPC_Heat.BPC_Heat_C|GetBoxes (Actor|GetComponentbyClass OtherActor "/Game/Main/Game/Components/BPC_Heat.BPC_Heat_C")) self))))

(event OnComponentEndOverlap(Box)
  (params (OverlappedComponent :type Primitive%20Component%20Object%20Reference) (OtherActor :type Actor%20Object%20Reference) (OtherComp :type Primitive%20Component%20Object%20Reference) (OtherBodyIndex :type Integer))
  (Networking|SwitchHasAuthority
    (:Authority
      (Utilities|Array|RemoveItem (Variables|/Game/Main/Game/Components/BPC_Heat.BPC_Heat_C|GetBoxes (Actor|GetComponentbyClass OtherActor "/Game/Main/Game/Components/BPC_Heat.BPC_Heat_C")) self))))

(event EventBeginPlay)

(event Collision|EventActorBeginOverlap
  (params (OtherActor :type Actor%20Object%20Reference)))

(event EventTick
  (params (DeltaSeconds :type Float%20%28single-precision%29)))

(fn ConstructionScript)