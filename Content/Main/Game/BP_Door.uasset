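; BP_Door is a physics door that players holding the matching key can lock or unlock.
; Main interaction checks the player's Keys for KeyIndex, plays a sound for success or failure, and toggles IsLocked.
; A multicast event locks the physics constraint's swing or limits it to 90 degrees.
; PlayerHit multicasts a force at the impact point, pushing the door mesh.
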(event Custom|PushDoor_Multicast
  (params (Force :type Vector) (Location :type Vector))
  (Class|PrimitiveComponent|AddForceatLocation (Variables|Default|GetDoorMesh) Force Location "None"))

(event Custom|SetDoorState_Multicast
  (params (IsLocked :type Boolean))
  (bind _physicsconstraint (Variables|Default|GetPhysicsConstraint))
  (if IsLocked
    (Class|PhysicsConstraintComponent|SetAngularOrientationTarget _physicsconstraint (Math|Rotator|MakeRotator 0.0 0.0 0.0))
    (Class|PhysicsConstraintComponent|SetAngularSwing1Limit (Variables|Default|GetPhysicsConstraint) "ACM_Locked" 0.0)
    (else
      (Class|PhysicsConstraintComponent|SetAngularOrientationTarget _physicsconstraint (Math|Rotator|MakeRotator 0.0 0.0 0.0))
      (Class|PhysicsConstraintComponent|SetAngularSwing1Limit (Variables|Default|GetPhysicsConstraint) "ACM_Limited" 9e+01))))

(event EventBeginPlay)

(event Collision|EventActorBeginOverlap
  (params (OtherActor :type Actor%20Object%20Reference)))

(event EventTick
  (params (DeltaSeconds :type Float%20%28single-precision%29)))

(event EventOnMainInteraction
  (params (Player :type PCC%20Game%20Object%20Reference))
  (bind _keys (Variables|/Game/Main/Game/PCC_Game.PCC_Game_C|GetKeys Player))
  (bind _keyindex (Variables|Default|GetKeyIndex))
  (bind _returnvalue (Utilities|Array|ContainsItem _keys _keyindex))
  (Audio|PlaySoundatLocation (select _returnvalue "/Engine/VREditor/Sounds/UI/Click_on_Button.Click_on_Button" "/Engine/VREditor/Sounds/UI/Camera_Shutter.Camera_Shutter") (Transformation|GetWorldLocation (Variables|Default|GetDoorMesh)) "0, 0, 0" 1.0 1.0 0.0 0 0 0 0)
  (if _returnvalue
    (if (Variables|Default|GetIsLocked)
      (Variables|Default|SetIsLocked false)
      (CallFunction|SetDoorStateMulticast false)
      (else
        (Variables|Default|SetIsLocked true)
        (CallFunction|SetDoorStateMulticast true)))))

(event EventPlayerHit
  (params (Player :type PCC%20Game%20Object%20Reference) (Direction :type Vector :default "0, 0, 0") (ImpactPoint :type Vector :default "0, 0, 0") (Force :type Integer))
  (CallFunction|PushDoorMulticast (* Direction Force) ImpactPoint))

(fn ConstructionScript)