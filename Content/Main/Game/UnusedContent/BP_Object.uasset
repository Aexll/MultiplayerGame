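; Grabbable physics prop that a character can carry in its hand and release.
; Grabed records the holder, turns off mesh simulation, limits collision to physics only, zeroes the actor transform and snaps the mesh to the character's Handsocket.
; UnGrabed restores physics and collision, detaches the actor and clears the holder.
; Collision is a stub returning true; its directional box traces and other force and placement experiments are unreachable.
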(event Custom|Grabed
  (params (Character :type PCC%20Object%20Reference))
  (bind _staticmesh (Variables|Default|GetStaticMesh))
  (Variables|Default|SetWhoGrab Character)
  (Variables|Default|SetIsGrab true)
  (Physics|SetSimulatePhysics _staticmesh false)
  (Collision|SetCollisionEnabled _staticmesh "PhysicsOnly")
  (Transformation|SetActorLocation "0, 0, 0" false false)
  (Transformation|SetActorRotation "0, 0, 0")
  (Transformation|AttachComponentToComponent (Variables|Default|GetStaticMesh) (Variables|/Script/Engine.Character|GetMesh Character) "Handsocket" "SnapToTarget" "SnapToTarget" "SnapToTarget" true))

(event Custom|UnGrabed
  (bind _staticmesh (Variables|Default|GetStaticMesh))
  (Physics|SetSimulatePhysics _staticmesh true)
  (Collision|SetCollisionEnabled _staticmesh "QueryAndPhysics")
  (Transformation|DetachFromActor "KeepWorld" "KeepRelative" "KeepRelative")
  (Variables|Default|SetWhoGrab 0)
  (Variables|Default|SetIsGrab false))

(event EventBeginPlay)

(event Collision|EventActorBeginOverlap
  (params (OtherActor :type Actor%20Object%20Reference)))

(event EventTick
  (params (DeltaSeconds :type Float%20%28single-precision%29)))

(fn ConstructionScript)

(fn Collision
  (params (Direction :type ETouchSwipeDirection%20Enum :default "None") (Width :type Float%20%28double-precision%29))
  (return true))