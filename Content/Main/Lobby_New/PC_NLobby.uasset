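; Player controller for the multiplayer lobby, handling lobby UI, player initialization, game launch and leaving.
; On spawn it creates the lobby HUD and an M-toggled menu, loads player info from the game instance, then notifies GM_NLobby after a short delay.
; It forwards player lists to the HUD and launch requests to the game mode.
; When the host leaves, other players' controllers leave first; sessions are destroyed before returning to MainMenu, and also on EndPlay.
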(event Custom|SetPlayerInfo
  (params (Info :type Player%20Info%20Structure))
  ;[1 0.1515 0] On spawn
  (Variables|Default|SetPlayerInfo Info))

(event Custom|LaunchGame
  (bind _asgm_nlobby (Utilities|Casting|CastToGM_NLobby (Game|GetGameMode)))
  (Default|LaunchGame _asgm_nlobby))

(event Custom|HUDMaking
  ;[1 0.09136 0] Lobby
  (bind _returnvalue (UserInterface|CreateWidget "/Game/Main/Lobby_New/HUDs/HUD_NLobby.HUD_NLobby_C" self))
  (bind _output_get (Variables|Default|SetHUD_Lobby _returnvalue))
  (UserInterface|Viewport|AddtoViewport _output_get 0)
  ;[1 0.09136 0] Menu
  (bind _returnvalue_2 (UserInterface|CreateWidget "/Game/Main/HUD_Menu.HUD_Menu_C" self))
  (Variables|Default|SetHUD_Menu _returnvalue_2))

(event Custom|LeaveGame
  (Networking|SwitchHasAuthority
    (:Authority
      ;[0 0.1697 1] Quit all authers players
      (for _array_element (Variables|/Script/Engine.GameStateBase|GetPlayerArray (Game|GetGameState))
        (if (!= _array_element (Variables|GetPlayerState self))
          (bind _asps_lobby (Utilities|Casting|CastToPS_Lobby _array_element))
          (bind _aspc_nlobby (Utilities|Casting|CastToPC_NLobby (Game|GetPlayerController _asps_lobby)))
          (CallFunction|LeaveGame _aspc_nlobby))))
    (:Remote
      _))
  ;[1 0 0.5615] Quit the lobby
  (|DestroySession self
    (:OnSuccess
      (Game|OpenLevel(byObjectReference) "/Game/Main/Menu/Map/MainMenu.MainMenu"))))

(event Custom|OnPlayerSpawn
  ;[1 0.1515 0] On spawn
  (Utilities|FlowControl|Sequence
    (:then_0
      (CallFunction|HUDMaking))
    (:then_1
      (bind _asgi (Utilities|Casting|CastToGI (Game|GetGameInstance)))
      (CallFunction|SetPlayerInfo (Default|LoadPlayerInfo _asgi))
      (Utilities|FlowControl|Delay 0.2)
      (CallFunction|DoneInit))))

(event Custom|DoneInit
  ;[1 0.1515 0] On spawn
  (bind _asgm_nlobby (Utilities|Casting|CastToGM_NLobby (Game|GetGameMode)))
  (Default|OnPlayerDoneInit _asgm_nlobby self))

(event Custom|ActLobbyHUD
  (params (PlayersInfos :type Array%20of%20Player%20Info%20Structures))
  (Default|GeneratePins (Variables|Default|GetHUD_Lobby) PlayersInfos))

(event EventBeginPlay)

(event EventTick
  (params (DeltaSeconds :type Float%20%28single-precision%29)))

(event EventEndPlay
  (params (EndPlayReason :type EEndPlayReason%20Enum :default "Destroyed"))
  ;[1 0 0] On quiting the game
  (|DestroySession self))

(event Input|KeyboardEvents|M
  (params (Key :type Key%20Structure :default "None"))
  (bind _hud_menu (Variables|Default|GetHUD_Menu))
  ;[1 0 0.346] Menu
  (:Pressed
    (if (UserInterface|Viewport|IsinViewport (Variables|Default|GetHUD_Menu))
      (Widget|RemovefromParent _hud_menu)
      (else
        (UserInterface|Viewport|AddtoViewport _hud_menu 0)))))

(fn ConstructionScript)